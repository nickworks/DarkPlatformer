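; Wall node mesher that builds a wall or doorway from randomized block mesh instances.
; Init picks the layout by node type: a full wall, or two sides and a top around a door opening for open and locked passages alike.
; FillRegionWithBlocks fits a block grid to each region, randomly leaving gaps.
; A random stream jitters depth, thickness and rotation, summing several rolls per angle for center-weighted tilt.
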(fn `Fill Region With Blocks`
  (params (`Region Thickness` :type "Float (double-precision)") (`Region Width` :type "Float (double-precision)") (`Region Height` :type "Float (double-precision)") (`Y Min` :type "Float (double-precision)") (`Z Min` :type "Float (double-precision)"))
  (locals (`Block width` :type "Float (double-precision)" :default 0.0) (`Block height` :type "Float (double-precision)" :default 0.0) (`Columns of blocks` :type Integer :default 0) (`Rows of blocks` :type Integer :default 0) (Y :type "Float (double-precision)") (Z :type "Float (double-precision)"))
  (bind _random_stream (`self.Random Stream`))
  (bind _returnvalue (`KismetMathLibrary.RandomFloatInRangeFromStream` -0.5 0.5 (`self.Random Stream`)))
  (bind _returnvalue_2 (`KismetMathLibrary.RandomFloatInRangeFromStream` -2.0 2.0 (`self.Random Stream`)))
  (bind _output_get (set `local.Columns of blocks` (`KismetMathLibrary.FTrunc` (/ (`local.Region Width`) (`self.target block width`)))))
  (set `local.Block width` (/ (`local.Region Width`) (`KismetMathLibrary.Conv_IntToDouble` _output_get)))
  (bind _output_get_2 (set `local.Rows of blocks` (`KismetMathLibrary.FTrunc` (/ (`local.Region Height`) (`self.target block height`)))))
  (set `local.Block height` (/ (`local.Region Height`) (`KismetMathLibrary.Conv_IntToDouble` _output_get_2)))
  (set `local.Y` (+ (`local.Y Min`) (/ (`local.Block width`) -2.0)))
  (set `local.Z` (+ (`local.Z Min`) (/ (`local.Block height`) 2.0)))
  (for _ (range 1 (+ (`local.Rows of blocks`) 1))
    (for _ (range 1 (+ (`local.Columns of blocks`) 1))
      (set `local.Y` (+ (`local.Y`) (`local.Block width`)))
      (if (`KismetMathLibrary.RandomBoolWithWeightFromStream` 0.85 _random_stream)
        (`self.AddInstance` (`KismetMathLibrary.MakeTransform` (`KismetMathLibrary.MakeVector` (`KismetMathLibrary.RandomFloatInRangeFromStream` 0.0 20.0 _random_stream) (`local.Y`) (`local.Z`)) (`KismetMathLibrary.MakeRotator` 0.0 (+ _returnvalue _returnvalue _returnvalue _returnvalue) (+ _returnvalue_2 _returnvalue_2 _returnvalue_2 _returnvalue_2)) (`KismetMathLibrary.MakeVector` (* (`self.thickness`) (`KismetMathLibrary.RandomFloatInRangeFromStream` 1.0 2.0 (`self.Random Stream`))) (/ (`local.Block width`) 100.0) (/ (`local.Block height`) 100.0))))))
    (set `local.Z` (+ (`local.Z`) (`local.Block height`)))
    (set `local.Y` (+ (`local.Y Min`) (/ (`local.Block width`) -2.0)))))

(fn `Init`
  (params (`Wall Node Type` :type "/Game/Blueprints/WallNodeTypes Enum" :default "NewEnumerator0") (`Node Width` :type "Float (double-precision)" :default 20.0) (height :type "Float (double-precision)" :default 4.0) (thickness :type "Float (double-precision)" :default 0.5))
  (bind _returnvalue (* (`self.height of door`) 100.0))
  (bind _returnvalue_2 (* (`self.thickness`) 100.0))
  (bind _returnvalue_3 (/ (- (`self.width`) (`self.width of door`)) 2.0))
  (bind _returnvalue_4 (* _returnvalue_3 100.0))
  (set `self.width` `Node Width`)
  (set `self.height` height)
  (set `self.thickness` thickness)
  (bind _output_get (set `self.Wall Node Type` `Wall Node Type`))
  (switch `/Game/Blueprints/WallNodeTypes` _output_get
    (:`NewEnumerator0`
      (`self.Fill Region With Blocks` (* (`self.thickness`) 100.0) (* (`self.width`) 100.0) (* (`self.height`) 100.0) 0.0 0.0))
    (:`NewEnumerator1`
      (`self.Fill Region With Blocks` _returnvalue_2 _returnvalue_4 _returnvalue 0.0 0.0 :!label _label)
      (`self.Fill Region With Blocks` _returnvalue_2 _returnvalue_4 _returnvalue (* (+ _returnvalue_3 (`self.width of door`)) 100.0) 0.0)
      (`self.Fill Region With Blocks` (* (`self.thickness`) 100.0) (* (`self.width`) 100.0) (* (- (`self.height`) (`self.height of door`)) 100.0) 0.0 (* (`self.height of door`) 100.0)))
    (:`NewEnumerator3`
      (goto _label))))