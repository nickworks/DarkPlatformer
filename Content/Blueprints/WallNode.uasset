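; WallNode is a wall segment actor that builds either a solid wall or a wall with a doorway, based on its node type.
; The construction script calls Init, which stores type and width, then adds scaled, offset instances to an InstancedStaticMesh.
; Solid walls use one instance, while passages use two equal side pieces and a lintel around a centered opening.
; Locked-door passages currently share the open passage geometry, with no door added.
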(fn `Init`
  (params (`Node Type` :type "/Game/Blueprints/WallNodeTypes Enum" :default "NewEnumerator0") (`Node Width` :type "Float (double-precision)" :default 20.0))
  (bind _height_of_door (`self.height of door`))
  (bind _width (`self.width`))
  (bind _height (`self.height`))
  (bind _thickness (`self.thickness`))
  (bind _thickness_2 (`self.thickness`))
  (bind _width_2 (`self.width`))
  (bind _thickness_3 (`self.thickness`))
  (bind _returnvalue (- (`self.height`) (`self.height of door`)))
  (bind _returnvalue_2 (* _thickness_2 50.0))
  (bind _returnvalue_3 (* _height_of_door 50.0))
  (bind _returnvalue_4 (/ (- (`self.width`) (`self.width of door`)) 2.0))
  (bind _returnvalue_5 (* _returnvalue_4 50.0))
  (set `self.width` `Node Width`)
  (bind _output_get (set `self.Wall Node Type` `Node Type`))
  (switch `/Game/Blueprints/WallNodeTypes` _output_get
    (:`NewEnumerator0`
      (`InstancedStaticMeshComponent.AddInstance` (`self.InstancedStaticMesh`) (`KismetMathLibrary.MakeTransform` (`KismetMathLibrary.MakeVector` (* _thickness 50.0) (* _width 50.0) (* _height 50.0)) (struct) (`KismetMathLibrary.MakeVector` _thickness _width _height))))
    (:`NewEnumerator1`
      (`InstancedStaticMeshComponent.AddInstance` (`self.InstancedStaticMesh`) (`KismetMathLibrary.MakeTransform` (`KismetMathLibrary.MakeVector` _returnvalue_2 _returnvalue_5 _returnvalue_3) (struct) (`KismetMathLibrary.MakeVector` _thickness_2 _returnvalue_4 _height_of_door)) :!label _label)
      (`InstancedStaticMeshComponent.AddInstance` (`self.InstancedStaticMesh`) (`KismetMathLibrary.MakeTransform` (`KismetMathLibrary.MakeVector` _returnvalue_2 (- (* (`self.width`) 100.0) _returnvalue_5) _returnvalue_3) (struct) (`KismetMathLibrary.MakeVector` _thickness_2 _returnvalue_4 _height_of_door)))
      (`InstancedStaticMeshComponent.AddInstance` (`self.InstancedStaticMesh`) (`KismetMathLibrary.MakeTransform` (`KismetMathLibrary.MakeVector` (* _thickness_3 50.0) (* _width_2 50.0) (* (+ (`self.height of door`) (/ _returnvalue 2.0)) 100.0)) (struct) (`KismetMathLibrary.MakeVector` _thickness_3 _width_2 _returnvalue))))
    (:`NewEnumerator3`
      (goto _label))))

(fn `UserConstructionScript`
  (`self.Init` (`self.Wall Node Type`) (`self.width`)))