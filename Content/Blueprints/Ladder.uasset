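; Procedurally built climbable ladder that puts the first-person character on it on interact, if roughly facing the grip direction, and off on leaving its volume.
; Init sizes the colliders, builds instanced rails and rungs, tilts the pivot and adds two seeded wall-builder components below.
; Rungs are randomly skipped and jittered with summed randoms for bell-curve spread, but ignore the seeded stream.
; The construction script is empty, so building relies on Init.
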(event `self.Box-Front.OnComponentBeginOverlap`
  (params (OverlappedComponent :type "PrimitiveComponent Object Reference") (OtherActor :type "Actor Object Reference") (OtherComp :type "PrimitiveComponent Object Reference") (OtherBodyIndex :type Integer) (bFromSweep :type Boolean) (SweepResult :type "HitResult Structure (by ref)")))

(event `self.Box-Volume.OnComponentEndOverlap`
  (params (OverlappedComponent :type "PrimitiveComponent Object Reference") (OtherActor :type "Actor Object Reference") (OtherComp :type "PrimitiveComponent Object Reference") (OtherBodyIndex :type Integer))
  (bind _asfirst_person_character (cast `/Game/Blueprints/PlayerCharacter/FirstPersonCharacter` OtherActor))
  (`/Game/Blueprints/PlayerCharacter/FirstPersonCharacter.Off Ladder` _asfirst_person_character))

(event `/Game/Blueprints/SomethingThatCanBeInteractedWith.Player Attempted Interact`
  (params (Player :type "/Game/Blueprints/PlayerCharacter/FirstPersonCharacter Object Reference"))
  (bind _ascend_direction (`self.Ascend Direction`))
  (if (> (`KismetMathLibrary.Dot_VectorVector` (`self.GetActorForwardVector` Player) (`SceneComponent.GetForwardVector` (`self.Grip Direction`))) 0.25)
    (`/Game/Blueprints/PlayerCharacter/FirstPersonCharacter.On Ladder` Player (`SceneComponent.GetForwardVector` (`self.Grip Direction`)) (`SceneComponent.GetForwardVector` _ascend_direction) (`SceneComponent.K2_GetComponentLocation` _ascend_direction) 0.0)))

(fn `Init`
  (params (height :type "Float (double-precision)") (angle :type "Float (double-precision)") (seed :type Integer))
  (locals (`Height of Box` :type "Float (double-precision)" :default 0.0) (`Wall Height` :type "Float (double-precision)" :default 0.0) (`Wall Width` :type "Float (double-precision)" :default 0.0))
  (bind _random_stream (`self.Random Stream`))
  (set `self.height` height)
  (`KismetMathLibrary.SetRandomStreamSeed` (`self.Random Stream`) seed)
  (`self.Setup Colliders`)
  (`self.Make Rails`)
  (`self.Make Rungs`)
  (`SceneComponent.K2_SetRelativeRotation` (`self.ladder pivot`) (`KismetMathLibrary.MakeRotator` angle) false false)
  (set `local.Height of Box` (`KismetMathLibrary.RandomFloatInRangeFromStream` 1.0 10.0 (`self.Random Stream`)))
  (bind _output_get (set `local.Wall Height` (`KismetMathLibrary.Conv_IntToDouble` (`KismetMathLibrary.RandomIntegerInRangeFromStream` 3 10 (`self.Random Stream`)))))
  (set `local.Wall Width` (`KismetMathLibrary.Conv_IntToDouble` (`KismetMathLibrary.RandomIntegerInRangeFromStream` 2 4 (`self.Random Stream`))))
  (bind _returnvalue (* _output_get -100.0))
  (bind _returnvalue_2 (`AddComponent|NODE_AddBuilder_WallNodes-0` :`RelativeTransform` (`KismetMathLibrary.MakeTransform` (`KismetMathLibrary.MakeVector` 0.0 -100.0 _returnvalue))))
  (`/Game/Blueprints/ProceduralGeneration/Builder_WallNodes.Init` _returnvalue_2 "NewEnumerator0" (`local.Wall Width`) (`local.Wall Height`) 1.0 (`KismetMathLibrary.RandomIntegerFromStream` 1000000 (`self.Random Stream`)) false true)
  (bind _returnvalue_3 (`AddComponent|NODE_AddBuilder_WallNodes-1` :`RelativeTransform` (`KismetMathLibrary.MakeTransform` (`KismetMathLibrary.MakeVector` 0.0 (+ (* (`local.Wall Width`) 100.0) -100.0) _returnvalue))))
  (`/Game/Blueprints/ProceduralGeneration/Builder_WallNodes.Init` _returnvalue_3 "NewEnumerator0" (`KismetMathLibrary.RandomFloatInRangeFromStream` 5.0 15.0 _random_stream) (`local.Wall Height`) 0.75 (`KismetMathLibrary.RandomIntegerFromStream` 1000000 _random_stream) true false))

(fn `Make Rails`
  (`InstancedStaticMeshComponent.AddInstance` (`self.Rails - InstancedStaticMesh`) (`KismetMathLibrary.MakeTransform` (`KismetMathLibrary.MakeVector` (* (`self.width`) 50.0) 0.0 (* (`self.height`) 50.0)) (struct) (`KismetMathLibrary.MakeVector` 0.1 0.1 (`self.height`))))
  (`InstancedStaticMeshComponent.AddInstance` (`self.Rails - InstancedStaticMesh`) (`KismetMathLibrary.MakeTransform` (`KismetMathLibrary.MakeVector` (* (`self.width`) -50.0) 0.0 (* (`self.height`) 50.0)) (struct) (`KismetMathLibrary.MakeVector` 0.1 0.1 (`self.height`)))))

(fn `Make Rungs`
  (locals (rungs :type Integer) (z :type "Float (double-precision)"))
  (bind _returnvalue (`KismetMathLibrary.RandomFloatInRange` 0.02 0.05))
  (bind _returnvalue_2 (`KismetMathLibrary.RandomFloatInRange` -1.0 1.0))
  (bind _returnvalue_3 (`KismetMathLibrary.RandomFloatInRange` -2.0 2.0))
  (bind _returnvalue_4 (+ _returnvalue_2 _returnvalue_2 _returnvalue_2 _returnvalue_2))
  (bind _output_get (set `local.rungs` (`KismetMathLibrary.FTrunc` (/ (* (`self.height`) 100.0) (`self.ideal distance between rungs`)))))
  (set `local.z` 1.0)
  (for _index (range 1 _output_get)
    (if (`KismetMathLibrary.RandomBoolWithWeight` 0.8)
      (`InstancedStaticMeshComponent.AddInstance` (`self.Rungs - InstancedStaticMesh`) (`KismetMathLibrary.MakeTransform` (`KismetMathLibrary.MakeVector` _returnvalue_4 (* (`KismetMathLibrary.RandomFloatInRange` 3.0 5.0) (select `bool` (`KismetMathLibrary.RandomBoolWithWeight` 0.7) :`false` -1.0 :`true` 1.0 :!type "Float (single-precision)")) (+ (* _index (`self.ideal distance between rungs`)) _returnvalue_4 10.0)) (`KismetMathLibrary.MakeRotator` 0.0 (+ _returnvalue_3 _returnvalue_3 _returnvalue_3 _returnvalue_3)) (`KismetMathLibrary.MakeVector` (+ (`self.width`) 0.25) 0.05 (+ _returnvalue _returnvalue _returnvalue _returnvalue)))))))

(fn `Setup Colliders`
  (bind _box_collision (`self.Box-Collision`))
  (bind _returnvalue (* (`self.height`) 50.0))
  ;[1 1 1] volume
  (`BoxComponent.SetBoxExtent` (`self.Box-Volume`) (`KismetMathLibrary.MakeVector` (* (`self.width`) 50.0) 50.0 _returnvalue) true)
  (`SceneComponent.K2_SetRelativeLocation` (`self.Box-Volume`) (`KismetMathLibrary.MakeVector` 0.0 50.0 _returnvalue) false false)
  (`BoxComponent.SetBoxExtent` _box_collision (`KismetMathLibrary.MakeVector` (* (+ (`self.width`) 0.3) 50.0) 8.0 (* (`self.height`) 50.0)) true)
  (`SceneComponent.K2_SetRelativeLocation` _box_collision (`KismetMathLibrary.MakeVector` 0.0 0.0 (* (`self.height`) 50.0)) false false))

(fn `UserConstructionScript`
  (locals (rungs :type Integer) (z :type "Float (double-precision)")))