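; Procedurally generated dungeon room actor with one to three stacked floors.
; Construction seeds a local random stream from the ProceduralDungeon game mode's stream, then rolls random wall-segment types for each side of every floor.
; BeginPlay spawns four corner PillarNode actors of varied height, adds wall and floor builder components that receive the shared stream, and spawns a SanityCube above the room's origin.
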(event `self.ReceiveBeginPlay`
  (`self.MakePillars`)
  (`self.MakeWalls`)
  (`|SpawnActorFromClass` "/Game/Blueprints/SanityCube.SanityCube_C" (`KismetMathLibrary.MakeTransform` (+ (`self.K2_GetActorLocation`) (0.0 0.0 600.0))) "Undefined" "OverrideRootScale" null null))

(fn `Generate All Data`
  (locals (`Max floors` :type Integer))
  (bind _max_floors (`local.Max Floors`))
  (`KismetArrayLibrary.Array_Clear` (`self.Floors`))
  (bind _output_get (set `local.Max Floors` (`KismetMathLibrary.RandomIntegerInRangeFromStream` 1 3 (`self.random stream`))))
  (for _index (range 1 (+ _output_get 1))
    (bind _wall_pieces (`self.Generate Data - One Wall` _index _max_floors))
    (bind _wall_pieces_2 (`self.Generate Data - One Wall` _index _max_floors))
    (bind _wall_pieces_3 (`self.Generate Data - One Wall` _index _max_floors))
    (bind _wall_pieces_4 (`self.Generate Data - One Wall` _index _max_floors))
    (`KismetArrayLibrary.Array_Add` (`self.Floors`) (make `/Game/Blueprints/FourWalls` _wall_pieces _wall_pieces_2 _wall_pieces_3 _wall_pieces_4))))

(fn `Generate Data - One Wall`
  (params (Floor :type Integer) (`Max Floor` :type Integer))
  (returns (`Wall Pieces` :type "Array of /Game/Blueprints/NodeTypes_Wall Enum"))
  (locals (`Array of Wall Types` :type "Array of /Game/Blueprints/NodeTypes_Wall Enum") (`New Wall Node` :type "/Game/Blueprints/NodeTypes_Wall Enum"))
  (for _ (range 1 (+ (`KismetMathLibrary.RandomIntegerInRangeFromStream` 1 4 (`self.random stream`)) 1))
    (set `local.New Wall Node` (cast `/Game/Blueprints/NodeTypes_Wall` (`KismetMathLibrary.Conv_IntToByte` (`KismetMathLibrary.RandomIntegerInRangeFromStream` 0 (- (enumcount `/Game/Blueprints/NodeTypes_Wall`) 1) (`self.random stream`)))))
    (if (and (`|EnumEquality` (`local.New Wall Node`) "NewEnumerator7") (!= 0 (`local.Max Floor`)))
      (set `local.New Wall Node` "NewEnumerator0"))
    (`KismetArrayLibrary.Array_Add` (`local.Array of Wall Types`) (`local.New Wall Node`)))
  (return (`local.Array of Wall Types`)))

(fn `MakePillars`
  (locals (`Full Room Height` :type "Float (double-precision)" :default 0.0))
  (bind _returnvalue (* (`self.Room Width`) 50.0))
  (bind _returnvalue_2 (* (`self.Room Length`) 50.0))
  (bind _returnvalue_3 (* _returnvalue -1.0))
  (bind _returnvalue_4 (* _returnvalue_2 -1.0))
  (set `local.Full Room Height` (+ (* (`KismetArrayLibrary.Array_Length` (`self.Floors`)) (`self.Room Height`)) 3.0))
  (bind _returnvalue_5 (`|SpawnActorFromClass` "/Game/Blueprints/PillarNode.PillarNode_C" (`KismetMathLibrary.MakeTransform` (+ (`self.K2_GetActorLocation`) (`KismetMathLibrary.MakeVector` _returnvalue _returnvalue_2 50.0))) "Undefined" "OverrideRootScale" null null))
  (`/Game/Blueprints/PillarNode.Init` _returnvalue_5 (* (`local.Full Room Height`) (`KismetMathLibrary.RandomFloatInRangeFromStream` 1.0 1.25 (`self.random stream`))))
  (bind _returnvalue_6 (`|SpawnActorFromClass` "/Game/Blueprints/PillarNode.PillarNode_C" (`KismetMathLibrary.MakeTransform` (+ (`self.K2_GetActorLocation`) (`KismetMathLibrary.MakeVector` _returnvalue _returnvalue_4 50.0))) "Undefined" "OverrideRootScale" null null))
  (`/Game/Blueprints/PillarNode.Init` _returnvalue_6 (* (`local.Full Room Height`) (`KismetMathLibrary.RandomFloatInRangeFromStream` 1.0 1.25 (`self.random stream`))))
  (bind _returnvalue_7 (`|SpawnActorFromClass` "/Game/Blueprints/PillarNode.PillarNode_C" (`KismetMathLibrary.MakeTransform` (+ (`self.K2_GetActorLocation`) (`KismetMathLibrary.MakeVector` _returnvalue_3 _returnvalue_4 50.0))) "Undefined" "OverrideRootScale" null null))
  (`/Game/Blueprints/PillarNode.Init` _returnvalue_7 (* (`local.Full Room Height`) (`KismetMathLibrary.RandomFloatInRangeFromStream` 1.0 1.25 (`self.random stream`))))
  (bind _returnvalue_8 (`|SpawnActorFromClass` "/Game/Blueprints/PillarNode.PillarNode_C" (`KismetMathLibrary.MakeTransform` (+ (`self.K2_GetActorLocation`) (`KismetMathLibrary.MakeVector` _returnvalue_3 _returnvalue_2 50.0))) "Undefined" "OverrideRootScale" null null))
  (`/Game/Blueprints/PillarNode.Init` _returnvalue_8 (* (`local.Full Room Height`) (`KismetMathLibrary.RandomFloatInRangeFromStream` 1.0 1.25 (`self.random stream`)))))

(fn `MakeWalls`
  (locals (x :type "Float (double-precision)" :default 0.0) (y :type "Float (double-precision)" :default 0.0) (`step-x` :type "Float (double-precision)" :default 0.0) (`step-y` :type "Float (double-precision)") (z :type "Float (double-precision)") (`width of node` :type "Float (double-precision)" :default 0.0))
  (bind _returnvalue (- (`self.Room Length`) (`self.pillar width`)))
  (bind _returnvalue_2 (- (`self.Room Width`) (`self.pillar width`)))
  (bind _returnvalue_3 (- (`self.Room Width`) (`self.pillar width`)))
  (bind _returnvalue_4 (- (`self.Room Length`) (`self.pillar width`)))
  (set `local.z` 50.0)
  (for _array_element (`self.Floors`)
    (`|ExecutionSequence`
      (:`then_0`
        ;[1 1 1] North
        (set `local.x` (* _returnvalue_3 50.0))
        (set `local.y` (* (`self.Room Length`) 50.0))
        (bind (_north _east _south _west) (break `/Game/Blueprints/FourWalls` _array_element))
        (bind _output_get (set `local.width of node` (/ _returnvalue_3 (`KismetMathLibrary.Conv_IntToDouble` (`KismetArrayLibrary.Array_Length` _north)))))
        (set `local.step-x` (* _output_get -100.0))
        (set `local.step-y` 0.0)
        (for _array_element_2 _north
          (bind _returnvalue_5 (`AddComponent|NODE_AddWallNodeMesher-5` :`RelativeTransform` (`KismetMathLibrary.MakeTransform` (`KismetMathLibrary.MakeVector` (`local.x`) (`local.y`) (`local.z`)) (struct :`Yaw` 90.0))))
          (`/Game/Blueprints/Builder_WallNodes.Init` _returnvalue_5 _array_element_2 (`local.width of node`) (`self.Room Height`) (`self.Wall thickness`) (0.0 1.0 0.0) (`self.random stream`))
          (set `local.x` (+ (`local.x`) (`local.step-x`)))
          (set `local.y` (+ (`local.y`) (`local.step-y`)))))
      (:`then_1`
        ;[1 1 1] East
        (set `local.x` (* (`self.Room Width`) -50.0))
        (set `local.y` (* _returnvalue_4 -50.0))
        (bind _output_get_2 (set `local.width of node` (/ _returnvalue_4 (`KismetMathLibrary.Conv_IntToDouble` (`KismetArrayLibrary.Array_Length` _east)))))
        (set `local.step-x` 0.0)
        (set `local.step-y` (* _output_get_2 100.0))
        (for _array_element_3 _east
          (bind _returnvalue_6 (`AddComponent|NODE_AddWallNodeMesher-6` :`RelativeTransform` (`KismetMathLibrary.MakeTransform` (`KismetMathLibrary.MakeVector` (`local.x`) (`local.y`) (`local.z`)))))
          (`/Game/Blueprints/Builder_WallNodes.Init` _returnvalue_6 _array_element_3 (`local.width of node`) (`self.Room Height`) (`self.Wall thickness`) (-1.0 0.0 0.0) (`self.random stream`))
          (set `local.x` (+ (`local.x`) (`local.step-x`)))
          (set `local.y` (+ (`local.y`) (`local.step-y`)))))
      (:`then_2`
        ;[1 1 1] South
        (set `local.x` (* _returnvalue_2 50.0))
        (set `local.y` (* (`self.Room Length`) -50.0))
        (bind _output_get_3 (set `local.width of node` (/ _returnvalue_2 (`KismetMathLibrary.Conv_IntToDouble` (`KismetArrayLibrary.Array_Length` _south)))))
        (set `local.step-x` (* _output_get_3 -100.0))
        (set `local.step-y` 0.0)
        (for _array_element_4 _south
          (bind _returnvalue_7 (`AddComponent|NODE_AddWallNodeMesher-1` :`RelativeTransform` (`KismetMathLibrary.MakeTransform` (`KismetMathLibrary.MakeVector` (`local.x`) (`local.y`) (`local.z`)) (struct :`Yaw` 90.0))))
          (`/Game/Blueprints/Builder_WallNodes.Init` _returnvalue_7 _array_element_4 (`local.width of node`) (`self.Room Height`) (`self.Wall thickness`) (0.0 -1.0 0.0) (`self.random stream`))
          (set `local.x` (+ (`local.x`) (`local.step-x`)))
          (set `local.y` (+ (`local.y`) (`local.step-y`)))))
      (:`then_3`
        ;[1 1 1] West
        (set `local.x` (* (`self.Room Width`) 50.0))
        (set `local.y` (* _returnvalue -50.0))
        (bind _output_get_4 (set `local.width of node` (/ _returnvalue (`KismetMathLibrary.Conv_IntToDouble` (`KismetArrayLibrary.Array_Length` _west)))))
        (set `local.step-x` 0.0)
        (set `local.step-y` (* _output_get_4 100.0))
        (for _array_element_5 _west
          (bind _returnvalue_8 (`AddComponent|NODE_AddWallNodeMesher-2` :`RelativeTransform` (`KismetMathLibrary.MakeTransform` (`KismetMathLibrary.MakeVector` (`local.x`) (`local.y`) (`local.z`)))))
          (`/Game/Blueprints/Builder_WallNodes.Init` _returnvalue_8 _array_element_5 (`local.width of node`) (`self.Room Height`) (`self.Wall thickness`) (1.0 0.0 0.0) (`self.random stream`))
          (set `local.x` (+ (`local.x`) (`local.step-x`)))
          (set `local.y` (+ (`local.y`) (`local.step-y`)))))
      (:`then_4`
        (bind _returnvalue_9 (`AddComponent|NODE_AddBuilder_FloorNodes-0` :`RelativeTransform` (`KismetMathLibrary.MakeTransform` (`KismetMathLibrary.MakeVector` 0.0 0.0 (`local.z`)))))
        (`/Game/Blueprints/Builder_FloorNodes.Init` _returnvalue_9 (cast `/Game/Blueprints/NodeTypes_Floor` (`KismetMathLibrary.Conv_IntToByte` (`KismetMathLibrary.RandomIntegerInRangeFromStream` 0 (- (enumcount `/Game/Blueprints/NodeTypes_Floor`) 1) (`self.random stream`)))) (`self.Room Width`) (`self.Room Length`) (`self.random stream`)))
      (:`then_5`
        (set `local.z` (+ (`local.z`) (* (`self.Room Height`) 100.0)))))))

(fn `Setup random seed`
  (locals (Seed :type Integer :default 0))
  (bind _asprocedural_dungeon (cast `/Game/Blueprints/ProceduralDungeon` (`GameplayStatics.GetGameMode`)))
  (bind _output_get (set `local.Seed` (`KismetMathLibrary.RandomIntegerFromStream` 1000000 (`/Game/Blueprints/ProceduralDungeon.random stream` _asprocedural_dungeon))))
  (`KismetMathLibrary.SetRandomStreamSeed` (`self.random stream`) _output_get))

(fn `UserConstructionScript`
  (`self.Setup random seed`)
  (`self.Generate All Data`))