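; CrystalPlatform is a teleport destination with a slowly spinning Box component.
; On BeginPlay a timeline slowed to quarter speed drives the Box's relative yaw from its Spin track.
; TeleportActorToMe plays a close sound at the world origin, waits briefly, plays a click at the passed actor's location, then teleports that actor to the TeleportHere component without sweeping.
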(event `self.ReceiveBeginPlay`
  (`TimelineComponent.SetPlayRate` (`self.Timeline_0`) 0.25)
  (bind (_direction _spin) (`Timeline|Timeline_0`)
    (:`Update`
      (`SceneComponent.K2_SetRelativeRotation` (`self.Box`) (`KismetMathLibrary.MakeRotator` 0.0 0.0 _spin) false false))))

(event `Teleport Actor To Me`
  (params (`Actor to Teleport` :type "Actor Object Reference"))
  (`GameplayStatics.PlaySoundAtLocation` "/Engine/VREditor/Sounds/VR_close_Cue.VR_close_Cue" (0.0 0.0 0.0) (struct) 1.0 1.0 0.0 null null null)
  (`KismetSystemLibrary.Delay` 0.5)
  (`GameplayStatics.PlaySoundAtLocation` "/Engine/VREditor/Sounds/VR_click2_Cue.VR_click2_Cue" (`self.K2_GetActorLocation` `Actor to Teleport`) (struct) 1.0 1.0 0.0 null null null)
  (`self.K2_SetActorLocation` `Actor to Teleport` (`SceneComponent.K2_GetComponentLocation` (`self.Teleport Here`)) false true))

(fn `UserConstructionScript`)