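; PickupPillar is a pedestal that spawns an ItemType actor, attaches it to MovableBit and signals its state through a glow.
; Construction creates a dynamic Fire material on Cylinder1 with a starting color.
; Collider overlaps play or reverse a timeline that blends the glow color through HSV.
; The item's GotPickedUp event triggers a fade of the glow to black and stops further proximity reactions.
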(event `self.ReceiveBeginPlay`
  (bind _returnvalue (`|SpawnActorFromClass` (`self.ItemType`) (`KismetMathLibrary.MakeTransform` (+ (`self.K2_GetActorLocation`) (0.0 0.0 25.0))) "Undefined" "OverrideRootScale" self null))
  (add `/Game/Blueprints/InventoryItems/ItemAbilities/_ItemAbility.Got Picked Up` _returnvalue (delegate `Item Gone`))
  (`self.K2_AttachToComponent` _returnvalue (`self.Movable Bit`) "None" "KeepWorld" "KeepWorld" "KeepWorld" false))

(event `Item Gone`
  (set `self.Is Item Gone` true)
  (bind (_direction _fade_out) (`Timeline|Player Picked It Up`)
    (:`Update`
      (`MaterialInstanceDynamic.SetVectorParameterValue` (`self.Glow Material`) "Color" (`KismetMathLibrary.LinearColorLerp` (struct :`R` 5.882751 :`G` 0.505124 :`B` 10.0 :`A` 1.0) (struct) _fade_out)))))

(event `self.Collider.OnComponentBeginOverlap`
  (params (OverlappedComponent :type "PrimitiveComponent Object Reference") (OtherActor :type "Actor Object Reference") (OtherComp :type "PrimitiveComponent Object Reference") (OtherBodyIndex :type Integer) (bFromSweep :type Boolean) (SweepResult :type "HitResult Structure (by ref)"))
  (if (not (`self.Is Item Gone`))
    (bind (_direction _glow_amount) (`Timeline|Player Close Enough` :!label _label)
      (:`Update`
        (`MaterialInstanceDynamic.SetVectorParameterValue` (`self.Glow Material`) "Color" (`KismetMathLibrary.LinearColorLerpUsingHSV` (struct :`R` 0.473958 :`G` 0.021845 :`A` 6.686952) (struct :`R` 2.941375 :`G` 0.252562 :`B` 5.0 :`A` 1.0) _glow_amount))))))

(event `self.Collider.OnComponentEndOverlap`
  (params (OverlappedComponent :type "PrimitiveComponent Object Reference") (OtherActor :type "Actor Object Reference") (OtherComp :type "PrimitiveComponent Object Reference") (OtherBodyIndex :type Integer))
  (if (not (`self.Is Item Gone`))
    (goto _label :!via `Reverse`)))

(fn `UserConstructionScript`
  (bind _returnvalue (`PrimitiveComponent.CreateDynamicMaterialInstance` (`self.Cylinder1`) 0 "/Game/ArtStuff/Materials/fire.fire" "None"))
  (bind _output_get (set `self.Glow Material` _returnvalue))
  (`MaterialInstanceDynamic.SetVectorParameterValue` _output_get "Color" (struct :`R` 6.720939 :`G` 0.309773 :`A` 6.686952)))