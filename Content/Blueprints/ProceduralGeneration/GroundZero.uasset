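; GroundZero is a procedural generation Blueprint that scatters tall, stretched mesh instances across a square area below world zero.
; Init seeds a random stream, then loops to add instances to an InstancedStaticMesh in world space, so a given seed reproduces the layout.
; Each instance gets a random position and a random uniform horizontal scale, with a fixed, much larger vertical scale.
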(fn `Init`
  (params (seed :type Integer))
  (locals (scale :type "Float (double-precision)"))
  (bind _random_stream (`self.random stream`))
  (`KismetMathLibrary.SetRandomStreamSeed` _random_stream seed)
  (for _ (range 21)
    (bind _output_get (set `local.scale` (`KismetMathLibrary.RandomFloatInRangeFromStream` 2.0 4.0 _random_stream)))
    (`InstancedStaticMeshComponent.AddInstanceWorldSpace` (`self.InstancedStaticMesh`) (`KismetMathLibrary.MakeTransform` (`KismetMathLibrary.MakeVector` (`KismetMathLibrary.RandomFloatInRangeFromStream` -3000.0 3000.0 _random_stream) (`KismetMathLibrary.RandomFloatInRangeFromStream` -3000.0 3000.0 _random_stream) (`KismetMathLibrary.RandomFloatInRangeFromStream` -2000.0 -500.0 _random_stream)) (struct) (`KismetMathLibrary.MakeVector` _output_get _output_get 30.0)))))

(fn `UserConstructionScript`)