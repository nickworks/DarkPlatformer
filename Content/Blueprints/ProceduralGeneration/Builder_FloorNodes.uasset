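; Procedural floor builder that lays instanced stone blocks over a node's area, in a style chosen by FloorNodeType.
; Init uses a seeded stream to pick layout parameters or subdivide into random cells, and spawns a MonolithNode on top-floor perimeter nodes.
; BuildStoneFloor grids blocks, hollowing centres by Openness and randomly dropping stones.
; Summed randoms give bell-curve height and tilt jitter, while SinkAmount dishes stones toward the node's centre.
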(fn `Build Stone Floor`
  (params (`Region Width` :type "Float (double-precision)") (`Region Length` :type "Float (double-precision)") (`X Min` :type "Float (double-precision)") (`Y Min` :type "Float (double-precision)") (Openness :type "Float (double-precision)" :default 0.5) (`Percent of Stones Present` :type "Float (double-precision)") (SinkAmount :type "Float (double-precision)"))
  (locals (`Block width` :type "Float (double-precision)" :default 0.0) (`Block length` :type "Float (double-precision)" :default 0.0) (`Columns of blocks` :type Integer :default 0) (`Rows of blocks` :type Integer :default 0) (Y :type "Float (double-precision)") (X :type "Float (double-precision)"))
  (bind _rows_of_blocks (`local.Rows of blocks`))
  (bind _random_stream (`self.Random Stream`))
  (bind _columns_of_blocks (`local.Columns of blocks`))
  (bind _returnvalue (`KismetMathLibrary.RandomFloatInRangeFromStream` -0.5 0.5 (`self.Random Stream`)))
  (bind _returnvalue_2 (`KismetMathLibrary.RandomFloatInRangeFromStream` 0.0 1.0 _random_stream))
  (bind _returnvalue_3 (`KismetMathLibrary.Lerp` 0.0 6.0 (`local.SinkAmount`)))
  (bind _returnvalue_4 (`KismetMathLibrary.RandomFloatInRangeFromStream` -1.0 1.0 (`self.Random Stream`)))
  (bind _returnvalue_5 (+ _returnvalue_4 _returnvalue_4 _returnvalue_4 _returnvalue_4))
  (bind _returnvalue_6 (+ (/ (`local.Openness`) 2.0) 0.5))
  (bind _returnvalue_7 (`KismetMathLibrary.MakeVector` (`local.X`) (`local.Y`) (+ _returnvalue_2 _returnvalue_2 _returnvalue_2 _returnvalue_2)))
  (bind _output_get (set `local.Columns of blocks` (`KismetMathLibrary.FTrunc` (/ (`local.Region Length`) (`self.target block height`)))))
  (bind _output_get_2 (set `local.Rows of blocks` (`KismetMathLibrary.FTrunc` (/ (`local.Region Width`) (`self.target block width`)))))
  (set `local.Block width` (/ (`local.Region Width`) (`KismetMathLibrary.Conv_IntToDouble` _output_get_2)))
  (set `local.Block length` (/ (`local.Region Length`) (`KismetMathLibrary.Conv_IntToDouble` _output_get)))
  (set `local.Y` (+ (`local.Y Min`) (/ (`local.Block width`) -2.0)))
  (set `local.X` (+ (`local.X Min`) (/ (`local.Block length`) 2.0)))
  (for _index (range 1 (+ _rows_of_blocks 1))
    (for _index_2 (range 1 (+ _columns_of_blocks 1))
      (set `local.Y` (+ (`local.Y`) (`local.Block width`)))
      (bind _returnvalue_8 (/ (`KismetMathLibrary.Conv_IntToDouble` (- _index_2 1)) (`KismetMathLibrary.Conv_IntToDouble` (- _columns_of_blocks 1))))
      (bind _returnvalue_9 (/ (`KismetMathLibrary.Conv_IntToDouble` (- _index 1)) (`KismetMathLibrary.Conv_IntToDouble` (- _rows_of_blocks 1))))
      (if (or (<= _returnvalue_8 (- 1.0 _returnvalue_6)) (>= _returnvalue_8 _returnvalue_6) (<= _returnvalue_9 (- 1.0 _returnvalue_6)) (>= _returnvalue_9 _returnvalue_6))
        (if (`KismetMathLibrary.RandomBoolWithWeightFromStream` (`local.Percent of Stones Present`) _random_stream)
          (`self.AddInstance` (`KismetMathLibrary.MakeTransform` (+ _returnvalue_7 (* (`KismetMathLibrary.Vector_Up`) (`KismetMathLibrary.Lerp` 0.0 _returnvalue_3 (/ (`KismetMathLibrary.VSize` _returnvalue_7) 15.0))) (`KismetMathLibrary.MakeVector` 0.0 0.0 (* _returnvalue_3 -100.0))) (`KismetMathLibrary.MakeRotator` _returnvalue_5 _returnvalue_5 (+ _returnvalue _returnvalue _returnvalue _returnvalue)) (`KismetMathLibrary.MakeVector` (/ (`local.Block width`) 100.0) (/ (`local.Block length`) 100.0) (`self.thickness`)))))))
    (set `local.X` (+ (`local.X`) (`local.Block length`)))
    (set `local.Y` (+ (`local.Y Min`) (/ (`local.Block width`) -2.0)))))

(fn `Init`
  (params (`Floor Node Type` :type "/Game/Blueprints/ProceduralGeneration/NodeTypes_Floor Enum" :default "NewEnumerator1") (Width :type "Float (double-precision)" :default 100.0) (Length :type "Float (double-precision)" :default 100.0) (`Random Stream` :type "RandomStream Structure") (`Floor Index` :type Integer) (`Num of Floors` :type Integer))
  (locals (`Width in CM` :type "Float (double-precision)" :default 100.0) (`Length in CM` :type "Float (double-precision)" :default 0.0) (rows :type Integer :default 0) (cols :type Integer :default 0) (`cell width` :type "Float (double-precision)" :default 0.0) (`cell length` :type "Float (double-precision)" :default 0.0))
  (bind _width_in_cm (`local.Width in CM`))
  (bind _length_in_cm (`local.Length in CM`))
  (bind _width_in_cm_2 (`local.Width in CM`))
  (bind _length_in_cm_2 (`local.Length in CM`))
  (bind _width_in_cm_3 (`local.Width in CM`))
  (bind _length_in_cm_3 (`local.Length in CM`))
  (bind _random_stream (`self.Random Stream`))
  (bind _random_stream_2 (`self.Random Stream`))
  (bind _random_stream_3 (`self.Random Stream`))
  (bind _width_in_cm_4 (`local.Width in CM`))
  (bind _length_in_cm_4 (`local.Length in CM`))
  (bind _returnvalue (`KismetMathLibrary.RandomIntegerInRangeFromStream` 2 4 (`self.Random Stream`)))
  (set `local.Width in CM` (* Width 100.0))
  (set `local.Length in CM` (* Length 100.0))
  (`KismetMathLibrary.SetRandomStreamSeed` (`self.Random Stream`) (`KismetMathLibrary.RandomIntegerFromStream` 1000000 `Random Stream`))
  (bind _output_get (set `self.Floor Node Type` `Floor Node Type`))
  (switch `/Game/Blueprints/ProceduralGeneration/NodeTypes_Floor` _output_get
    (:`NewEnumerator1`
      ;[1 1 1] Subdivided
      (set `local.rows` _returnvalue :!label _label)
      (set `local.cols` _returnvalue)
      (set `local.cell width` (/ (`local.Width in CM`) (`KismetMathLibrary.Conv_IntToDouble` (`local.rows`))))
      (set `local.cell length` (/ (`local.Length in CM`) (`KismetMathLibrary.Conv_IntToDouble` (`local.cols`))))
      (for _index (range 1 (+ (`local.rows`) 1))
        (for _index_2 (range 1 (+ (`local.cols`) 1))
          (if (`KismetMathLibrary.RandomBoolWithWeightFromStream` 0.75 (`self.Random Stream`))
            (`self.Build Stone Floor` (`local.cell width`) (`local.cell length`) (- (* (- _index 1) (`local.cell width`)) (/ (`local.Width in CM`) 2.0)) (- (* (- _index_2 1) (`local.cell length`)) (/ (`local.Length in CM`) 2.0)) (`KismetMathLibrary.RandomFloatInRangeFromStream` 0.0 0.1 _random_stream_2) (`KismetMathLibrary.RandomFloatInRangeFromStream` 0.5 0.9 _random_stream_2) (`KismetMathLibrary.RandomFloatInRangeFromStream` 0.0 0.5 _random_stream_2))))))
    (:`NewEnumerator0`
      ;[1 1 1] Solid
      (`self.Build Stone Floor` _width_in_cm _length_in_cm (/ _width_in_cm -2.0) (/ _length_in_cm -2.0) 0.0 1.0 (`KismetMathLibrary.RandomFloatInRangeFromStream` 0.0 0.5 (`self.Random Stream`))))
    (:`NewEnumerator4`
      ;[1 1 1] Sketchy
      (`self.Build Stone Floor` _width_in_cm_4 _length_in_cm_4 (/ _width_in_cm_4 -2.0) (/ _length_in_cm_4 -2.0) 0.0 (`KismetMathLibrary.RandomFloatInRangeFromStream` 0.4 0.8 _random_stream_3) (`KismetMathLibrary.RandomFloatInRangeFromStream` 0.1 0.5 _random_stream_3)))
    (:`NewEnumerator2`
      ;[1 1 1] Perimeter
      (`self.Build Stone Floor` _width_in_cm_3 _length_in_cm_3 (/ _width_in_cm_3 -2.0) (/ _length_in_cm_3 -2.0) (`KismetMathLibrary.RandomFloatInRangeFromStream` 0.5 1.0 (`self.Random Stream`)) 0.9)
      (if (== (+ (`local.Floor Index`) 1) (`local.Num of Floors`))
        (`|SpawnActorFromClass` "/Game/Blueprints/ProceduralGeneration/MonolithNode.MonolithNode_C" (`KismetMathLibrary.MakeTransform` (`self.K2_GetComponentLocation`)) "Undefined" "OverrideRootScale" null null)))
    (:`NewEnumerator3`
      (goto _label))
    (:`NewEnumerator5`
      ;[1 1 1] Lowered
      (`self.Build Stone Floor` _width_in_cm_2 _length_in_cm_2 (/ _width_in_cm_2 -2.0) (/ _length_in_cm_2 -2.0) (`KismetMathLibrary.RandomFloatInRangeFromStream` 0.0 0.5 _random_stream) (`KismetMathLibrary.RandomFloatInRangeFromStream` 0.4 0.8 _random_stream) (`KismetMathLibrary.RandomFloatInRangeFromStream` 0.4 1.0 _random_stream) :!label _label_2))
    (:`NewEnumerator6`
      (goto _label_2))))