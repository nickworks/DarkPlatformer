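; MonolithNode is a procedural generation Blueprint that scatters its Crystal component to a random raised position around its origin.
; The Construction Script picks a random angle, radial distance and height from a random stream, converting polar coordinates into the crystal's relative location.
; The stream is reseeded with an unseeded random integer on each construction, so placement changes whenever the script reruns.
; BeginPlay is empty.
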(event `self.ReceiveBeginPlay`)

(fn `UserConstructionScript`
  (locals (angle :type "Float (double-precision)" :default 0.0) (distance :type "Float (double-precision)" :default 0.0))
  (bind _random_stream (`self.random stream`))
  (`KismetMathLibrary.SetRandomStreamSeed` (`self.random stream`) (`KismetMathLibrary.RandomInteger` 1000000))
  (bind _output_get (set `local.angle` (`KismetMathLibrary.RandomFloatInRangeFromStream` 0.0 360.0 _random_stream)))
  (bind _output_get_2 (set `local.distance` (`KismetMathLibrary.RandomFloatInRangeFromStream` 900.0 2000.0 _random_stream)))
  (`SceneComponent.K2_SetRelativeLocation` (`self.Crystal`) (`KismetMathLibrary.MakeVector` (* _output_get_2 (`KismetMathLibrary.DegCos` _output_get)) (* _output_get_2 (`KismetMathLibrary.DegSin` _output_get)) (`KismetMathLibrary.RandomFloatInRangeFromStream` 1700.0 2400.0 (`self.random stream`))) false false))