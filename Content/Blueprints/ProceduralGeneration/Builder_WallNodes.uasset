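; Procedural wall segment builder that, from a seeded stream and node type, builds stone block walls, collapsing walls, passages, doorways, torch walls, ladders or T-walls.
; Regions fill with jittered instanced blocks, thinning with height on top segments unless forced full; crumbling fills narrow row by row.
; Passages frame an opening and return an attach point used to spawn doors, side rooms and ladders.
; T-walls spawn a perpendicular child wall.
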(fn `Attach Door At`
  (params (`Attach Point` :type "Transform Structure") (width :type "Float (double-precision)" :default 200.0) (height :type "Float (double-precision)" :default 300.0) (`Locked?` :type Boolean))
  (bind _returnvalue (`|SpawnActorFromClass` "/Game/Blueprints/DoorBp.DoorBp_C" `Attach Point` "Undefined" "OverrideRootScale" null null))
  (`/Game/Blueprints/DoorBp.Init` _returnvalue width height `Locked?`))

(fn `Attach Side Room At`
  (params (`Attach Point` :type "Transform Structure"))
  (bind _random_stream (`self.Random Stream`))
  (bind _returnvalue (`KismetMathLibrary.RandomFloatInRangeFromStream` 0.2 0.8 (`self.Random Stream`)))
  ;[1 1 1] Make Side Room
  (bind _returnvalue_2 (`|SpawnActorFromClass` "/Game/Blueprints/ProceduralGeneration/SideRoom.SideRoom_C" (`KismetMathLibrary.MakeTransform` (+ (.location `Attach Point`) (0.0 0.0 0.0)) (`KismetMathLibrary.MakeRotator` (* (.roll (.rotation `Attach Point`)) _returnvalue) (* (.pitch (.rotation `Attach Point`)) _returnvalue) (.yaw (.rotation `Attach Point`)))) "Undefined" "OverrideRootScale" null null))
  (`/Game/Blueprints/ProceduralGeneration/SideRoom.Init` _returnvalue_2 (`KismetMathLibrary.RandomFloatInRangeFromStream` 4.0 6.0 _random_stream) (`KismetMathLibrary.RandomFloatInRangeFromStream` 4.0 16.0 _random_stream) (`KismetMathLibrary.RandomIntegerFromStream` 1000000 _random_stream) -1.0))

(fn `Build Node As Collapsing Wall`
  (params (`Percent Blocks Present` :type "Float (double-precision)"))
  (`self.Fill Region with Crumbling Blocks` (* (`self.thickness`) 100.0) (* (`self.width`) 100.0) (* (`self.height`) 100.0) 0.0 0.0 `Percent Blocks Present`))

(fn `Build Node As Doorway to Side Room`
  (params (`Locked?` :type Boolean) (`Percent Blocks Present` :type "Float (double-precision)"))
  (locals (`door width` :type "Float (double-precision)" :default 0.0))
  (bind _output_get (set `local.door width` (* (`KismetMathLibrary.RandomFloatInRangeFromStream` 1.5 2.5 (`self.Random Stream`)) (`self.width of door`))))
  (bind _attach_point (`self.Build Node W/ Passageway + Attach Point` _output_get (`self.height of door`) (`KismetMathLibrary.RandomBoolFromStream` (`self.Random Stream`)) `Percent Blocks Present` (`KismetMathLibrary.Conv_IntToDouble` (`KismetMathLibrary.RandomIntegerInRangeFromStream` 0 5 (`self.Random Stream`)))))
  (`self.Attach Side Room At` _attach_point)
  (`self.Attach Door At` _attach_point (`local.door width`) (`self.height of door`) (`local.Locked?`)))

(fn `Build Node As Ladder`
  (params (`Percent Blocks Present` :type "Float (double-precision)"))
  (locals (`height of ladder` :type "Float (double-precision)" :default 0.0) (`angle of ladder` :type "Float (double-precision)") (`offset z` :type "Float (double-precision)" :default 0.0) (`offset x` :type "Float (double-precision)" :default 0.0) (`Passage Height` :type "Float (double-precision)" :default 4.0) (`Passage Width` :type "Float (double-precision)") (z :type "Float (double-precision)"))
  (bind _angle_of_ladder (`local.angle of ladder`))
  (bind _height_of_ladder (`local.height of ladder`))
  (bind _random_stream (`self.Random Stream`))
  (set `local.Passage Height` (`KismetMathLibrary.RandomFloatInRangeFromStream` 2.0 6.0 (`self.Random Stream`)))
  (set `local.Passage Width` (`KismetMathLibrary.RandomFloatInRangeFromStream` 1.5 4.0 (`self.Random Stream`)))
  (set `local.height of ladder` (`KismetMathLibrary.RandomFloatInRangeFromStream` 3.0 (/ (`self.height`) 2.0) _random_stream))
  (set `local.angle of ladder` (`KismetMathLibrary.RandomFloatInRangeFromStream` 5.0 10.0 _random_stream))
  (set `local.offset z` (* _height_of_ladder (`KismetMathLibrary.DegCos` _angle_of_ladder)))
  (set `local.offset x` (* _height_of_ladder (`KismetMathLibrary.DegSin` _angle_of_ladder)))
  ;[1 1 1] pick final z position of ladder
  (set `local.z` (`KismetMathLibrary.RandomFloatInRangeFromStream` (+ (`local.offset z`) 1.0) (- (`self.height`) (`local.Passage Height`)) (`self.Random Stream`)))
  (bind _attach_point (`self.Build Node W/ Passageway + Attach Point` (`local.Passage Width`) (`local.Passage Height`) (`KismetMathLibrary.RandomBoolWithWeightFromStream` 0.75 (`self.Random Stream`)) (`local.Percent Blocks Present`) (`local.z`)))
  (bind _returnvalue (`|SpawnActorFromClass` "/Game/Blueprints/Ladder.Ladder_C" (`KismetMathLibrary.MakeTransform` (`KismetMathLibrary.TransformLocation` _attach_point (* (`KismetMathLibrary.MakeVector` (+ (`self.thickness`) (`local.offset x`)) 0.0 (- 0.5 (`local.offset z`))) 100.0)) (`KismetMathLibrary.ComposeRotators` (struct :`Yaw` -90.0) (.rotation _attach_point))) "Undefined" "OverrideRootScale" null null))
  (`/Game/Blueprints/Ladder.Init` _returnvalue (`local.height of ladder`) (* (`local.angle of ladder`) -1.0) (`KismetMathLibrary.RandomIntegerFromStream` 1000000 (`self.Random Stream`))))

(fn `Build Node As T-Wall`
  (params (`Percent Blocks Present` :type "Float (double-precision)"))
  (bind _returnvalue (`self.K2_GetComponentToWorld`))
  (bind _random_stream (`self.Random Stream`))
  (`self.Fill Region With Blocks` (* (`self.thickness`) 100.0) (* (`self.width`) 100.0) (* (`self.height`) 100.0) 0.0 0.0 `Percent Blocks Present`)
  (bind _returnvalue_2 (`|SpawnActorFromClass` "/Game/Blueprints/ProceduralGeneration/Wall.Wall_C" (`KismetMathLibrary.MakeTransform` (`KismetMathLibrary.TransformLocation` _returnvalue (`KismetMathLibrary.MakeVector` 0.0 (* (`self.width`) 50.0) 0.0)) (`KismetMathLibrary.TransformRotation` _returnvalue (`KismetMathLibrary.MakeRotator` 0.0 0.0 (`KismetMathLibrary.SelectFloat` -90.0 90.0 (`KismetMathLibrary.RandomBoolFromStream` (`self.Random Stream`)))))) "Undefined" "OverrideRootScale" (`self.GetOwner`) null))
  (`/Game/Blueprints/ProceduralGeneration/Wall.Init` _returnvalue_2 (select `int` (`KismetMathLibrary.RandomIntegerInRangeFromStream` 0 2 _random_stream) :`0` "NewEnumerator0" :`1` "NewEnumerator1" :`2` "NewEnumerator7" :`3` "NewEnumerator0" :!type "/Game/Blueprints/ProceduralGeneration/NodeTypes_Wall Enum") (`KismetMathLibrary.Conv_IntToDouble` (`KismetMathLibrary.RandomIntegerInRangeFromStream` 3 8 _random_stream)) (`KismetMathLibrary.RandomFloatInRangeFromStream` 2.0 (`self.height`) _random_stream) 0.5 (`KismetMathLibrary.RandomIntegerFromStream` 100000 _random_stream) (`self.Is At Top`) false))

(fn `Build Node as Torch`
  (params (`Percent Blocks Present` :type "Float (double-precision)"))
  (`self.Fill Region With Blocks` (* (`self.thickness`) 100.0) (* (`self.width`) 100.0) (* (`self.height`) 100.0) 0.0 0.0 `Percent Blocks Present`))

(fn `Build Node As Wall`
  (params (`Has torch` :type Boolean) (`Percent Blocks Present` :type "Float (double-precision)"))
  (bind _returnvalue (`self.K2_GetComponentToWorld`))
  (`self.Fill Region With Blocks` (* (`self.thickness`) 100.0) (* (`self.width`) 100.0) (* (`self.height`) 100.0) 0.0 0.0 `Percent Blocks Present`)
  (if `Has torch`
    (`|SpawnActorFromClass` "/Game/Blueprints/Torch.Torch_C" (`KismetMathLibrary.MakeTransform` (`KismetMathLibrary.TransformLocation` _returnvalue (* (`KismetMathLibrary.MakeVector` (`self.thickness`) (/ (`self.width`) 2.0) 2.0) 100.0)) (.rotation _returnvalue)) "Undefined" "OverrideRootScale" null null)))

(fn `Build node as wide passageway`
  (params (`How many blocks wide` :type Integer) (`How many blocks high` :type Integer) (`Percent Blocks Present` :type "Float (double-precision)"))
  (bind _random_stream (`self.Random Stream`))
  (bind _returnvalue (`KismetMathLibrary.RandomFloatInRangeFromStream` 0.8 1.2 (`self.Random Stream`)))
  (`self.Build Node W/ Passageway + Attach Point` (* (/ (`self.target block width`) 100.0) _returnvalue (`KismetMathLibrary.Conv_IntToDouble` `How many blocks wide`)) (* (/ (`self.target block height`) 100.0) _returnvalue (`KismetMathLibrary.Conv_IntToDouble` `How many blocks high`)) (`KismetMathLibrary.RandomBoolFromStream` _random_stream) `Percent Blocks Present` (`KismetMathLibrary.Conv_IntToDouble` (`KismetMathLibrary.RandomIntegerInRangeFromStream` 0 5 _random_stream))))

(fn `Build Node W/ Passageway + Attach Point`
  (params (`Passage Width` :type "Float (double-precision)") (`Passage Height` :type "Float (double-precision)") (`Flip inside / outside` :type Boolean) (`Percent Blocks Present` :type "Float (double-precision)") (`Raised Up` :type "Float (double-precision)" :default 0.0))
  (returns (`Attach Point` :type "Transform Structure"))
  (locals (`Door Location` :type "Vector Structure" :default (0.0 0.0 0.0)) (`Door Rotation` :type "Rotator Structure" :default (struct)) (`Attach Pt` :type "Transform Structure"))
  (bind _percent_blocks_present (`local.Percent Blocks Present`))
  (bind _returnvalue (+ (`local.Passage Height`) (`local.Raised Up`)))
  (bind _returnvalue_2 (* (`local.Passage Height`) 100.0))
  (bind _returnvalue_3 (* (`self.thickness`) 100.0))
  (bind _returnvalue_4 (* (`local.Raised Up`) 100.0))
  (bind _returnvalue_5 (* (`self.thickness`) 100.0))
  (bind _returnvalue_6 (* (`self.width`) 100.0))
  (bind _returnvalue_7 (/ (- (`self.width`) (`local.Passage Width`)) 2.0))
  (bind _returnvalue_8 (* _returnvalue 100.0))
  (bind _returnvalue_9 (* _returnvalue_7 100.0))
  (bind _returnvalue_10 (* (- (`self.height`) _returnvalue) 100.0))
  (`self.Fill Region With Blocks` (* (`self.thickness`) 100.0) (* (`self.width`) 100.0) (* (`local.Raised Up`) 100.0) 0.0 0.0 (`local.Percent Blocks Present`)) ; Region below the door
  ;[1 1 1] Solid walls left and right of door
  (`self.Fill Region With Blocks` _returnvalue_5 _returnvalue_9 _returnvalue_2 0.0 _returnvalue_4 (`local.Percent Blocks Present`)) ; Region Left of Door
  (`self.Fill Region With Blocks` _returnvalue_5 _returnvalue_9 _returnvalue_2 (* (+ _returnvalue_7 (`local.Passage Width`)) 100.0) _returnvalue_4 (`local.Percent Blocks Present`)) ; Region Right of Door
  (if (`KismetMathLibrary.RandomBoolWithWeightFromStream` 0.7 (`self.Random Stream`))
    (`self.Fill Region With Blocks` _returnvalue_3 _returnvalue_6 _returnvalue_10 0.0 _returnvalue_8 _percent_blocks_present) ; Region Above Door
    (else
      (`self.Fill Region with Crumbling Blocks` _returnvalue_3 _returnvalue_6 _returnvalue_10 0.0 _returnvalue_8 _percent_blocks_present)))
  (bind _output_get (set `local.Attach Pt` (`KismetMathLibrary.MakeTransform` (`KismetMathLibrary.TransformLocation` (`self.K2_GetComponentToWorld`) (`KismetMathLibrary.MakeVector` 0.0 (* (`self.width`) 50.0) (* (`local.Raised Up`) 100.0))) (`KismetMathLibrary.ComposeRotators` (`KismetMathLibrary.MakeRotator` 0.0 0.0 (select `bool` (`local.Flip inside / outside`) :`true` 180.0 :!type "Float (single-precision)")) (`self.K2_GetComponentRotation`)))))
  (return _output_get))

(fn `Fill Region With Blocks`
  (params (`Region Thickness` :type "Float (double-precision)") (`Region Width` :type "Float (double-precision)") (`Region Height` :type "Float (double-precision)") (`Y Min` :type "Float (double-precision)") (`Z Min` :type "Float (double-precision)") (`Percent Blocks Present` :type "Float (double-precision)" :default 1.0))
  (locals (`Block width` :type "Float (double-precision)" :default 0.0) (`Block height` :type "Float (double-precision)" :default 0.0) (`Columns of blocks` :type Integer :default 0) (`Rows of blocks` :type Integer :default 0) (Y :type "Float (double-precision)") (Z :type "Float (double-precision)"))
  (bind _returnvalue (`KismetMathLibrary.RandomFloatInRangeFromStream` -0.5 0.5 (`self.Random Stream`)))
  (bind _returnvalue_2 (`KismetMathLibrary.RandomFloatInRangeFromStream` -2.0 2.0 (`self.Random Stream`)))
  (bind _output_get (set `local.Columns of blocks` (`KismetMathLibrary.FTrunc` (/ (`local.Region Width`) (`self.target block width`)))))
  (set `local.Block width` (/ (`local.Region Width`) (`KismetMathLibrary.Conv_IntToDouble` _output_get)))
  (bind _output_get_2 (set `local.Rows of blocks` (`KismetMathLibrary.FTrunc` (/ (`local.Region Height`) (`self.target block height`)))))
  (set `local.Block height` (/ (`local.Region Height`) (`KismetMathLibrary.Conv_IntToDouble` _output_get_2)))
  (set `local.Y` (+ (`local.Y Min`) (/ (`local.Block width`) -2.0)))
  (set `local.Z` (+ (`local.Z Min`) (/ (`local.Block height`) 2.0)))
  (for _index (range 1 (+ (`local.Rows of blocks`) 1))
    (for _ (range 1 (+ (`local.Columns of blocks`) 1))
      (set `local.Y` (+ (`local.Y`) (`local.Block width`)))
      (if (`self.Force 100%`)
        (`self.AddInstance` (`KismetMathLibrary.MakeTransform` (`KismetMathLibrary.MakeVector` (`KismetMathLibrary.RandomFloatInRangeFromStream` 0.0 20.0 (`self.Random Stream`)) (`local.Y`) (`local.Z`)) (`KismetMathLibrary.MakeRotator` 0.0 (+ _returnvalue _returnvalue _returnvalue _returnvalue) (+ _returnvalue_2 _returnvalue_2 _returnvalue_2 _returnvalue_2)) (`KismetMathLibrary.MakeVector` (* (`self.thickness`) (`KismetMathLibrary.RandomFloatInRangeFromStream` 1.0 2.0 (`self.Random Stream`))) (/ (`local.Block width`) 100.0) (/ (`local.Block height`) 100.0))) :!label _label)
        (elif (`KismetMathLibrary.RandomBoolWithWeightFromStream` (* (select `bool` (`self.Is At Top`) :`false` 0.95 :`true` (`KismetMathLibrary.FClamp` (- 1.0 (/ (`local.Z`) (* (`self.height`) 100.0))))) (`local.Percent Blocks Present`)) (`self.Random Stream`))
          (goto _label))))
    (set `local.Z` (+ (`local.Z`) (`local.Block height`)))
    (set `local.Y` (+ (`local.Y Min`) (/ (`local.Block width`) -2.0)))))

(fn `Fill Region with Crumbling Blocks`
  (params (`Region Thickness` :type "Float (double-precision)") (`Region Width` :type "Float (double-precision)") (`Region Height` :type "Float (double-precision)") (`Y Min` :type "Float (double-precision)") (`Z Min` :type "Float (double-precision)") (`Percent Blocks Present` :type "Float (double-precision)"))
  (locals (`Percent Remaining on Left` :type "Float (double-precision)") (`Percent Remaining on Right` :type "Float (double-precision)") (`Stacks of blocks` :type Integer :default 0) (`Rows of blocks` :type Integer))
  (bind _random_stream (`self.Random Stream`))
  (bind _target_block_height (`self.target block height`))
  (bind _target_block_height_2 (`self.target block height`))
  (bind _returnvalue (* (`local.Region Width`) (`local.Percent Remaining on Right`)))
  (bind _returnvalue_2 (`KismetMathLibrary.SelectFloat` (`KismetMathLibrary.RandomFloatInRangeFromStream` 0.6 0.99 _random_stream) (`KismetMathLibrary.RandomFloatInRangeFromStream` 0.95 0.99 _random_stream) (`KismetMathLibrary.RandomBoolWithWeightFromStream` 0.5 _random_stream)))
  (bind _returnvalue_3 (`KismetMathLibrary.FTrunc` (/ `Region Height` (`self.target block height`))))
  (if true
    (set `local.Rows of blocks` 0)
    (set `local.Percent Remaining on Left` 0.4)
    (set `local.Percent Remaining on Right` 0.4)
    (else
      (set `local.Rows of blocks` (`KismetMathLibrary.RandomIntegerInRangeFromStream` 1 3 (`self.Random Stream`)))
      (bind _output_get (set `local.Percent Remaining on Left` (`KismetMathLibrary.RandomFloatInRangeFromStream` 0.2 0.8 (`self.Random Stream`))))
      (set `local.Percent Remaining on Right` (- 1.0 _output_get))))
  (set `local.Stacks of blocks` _returnvalue_3)
  (for _index (range (+ _returnvalue_3 1))
    (`self.Fill Region With Blocks` (`local.Region Thickness`) (* (`local.Region Width`) (`local.Percent Remaining on Left`)) _target_block_height 0.0 (* _index _target_block_height) (`local.Percent Blocks Present`))
    (`self.Fill Region With Blocks` (`local.Region Thickness`) _returnvalue _target_block_height_2 (- (`local.Region Width`) _returnvalue) (* _index _target_block_height_2) (`local.Percent Blocks Present`))
    (if (>= _index (`local.Rows of blocks`))
      (set `local.Percent Remaining on Left` (`KismetMathLibrary.FClamp` (* _returnvalue_2 (`local.Percent Remaining on Left`))))
      (set `local.Percent Remaining on Right` (`KismetMathLibrary.FClamp` (* _returnvalue_2 (`local.Percent Remaining on Right`)))))))

(fn `Init`
  (params (`Wall Node Type` :type "/Game/Blueprints/ProceduralGeneration/NodeTypes_Wall Enum" :default "NewEnumerator0") (`Node Width` :type "Float (double-precision)" :default 20.0) (height :type "Float (double-precision)" :default 4.0) (thickness :type "Float (double-precision)" :default 0.5) (`wall seed` :type Integer) (`Is Top` :type Boolean) (`Force 100%` :type Boolean))
  (locals (`Percent Blocks Present` :type "Float (double-precision)"))
  (set `self.width` `Node Width`)
  (set `self.height` height)
  (set `self.thickness` thickness)
  (set `self.Is At Top` `Is Top`)
  (set `self.Force 100%` `Force 100%`)
  (`KismetMathLibrary.SetRandomStreamSeed` (`self.Random Stream`) `wall seed`)
  (bind _output_get (set `self.target block width` (`KismetMathLibrary.RandomFloatInRangeFromStream` 110.0 150.0 (`self.Random Stream`))))
  (set `self.target block height` (* _output_get 0.9))
  (bind _output_get_2 (set `self.Wall Node Type` `Wall Node Type`))
  (switch `/Game/Blueprints/ProceduralGeneration/NodeTypes_Wall` _output_get_2
    (:`NewEnumerator0`
      (`self.Build Node As Wall` false 1.0))
    (:`NewEnumerator1`
      (`self.Build node as wide passageway` 3 3 1.0))
    (:`NewEnumerator3`
      (`self.Build Node As Doorway to Side Room` true 1.0))
    (:`NewEnumerator11`
      (`self.Build Node As Doorway to Side Room` false 1.0))
    (:`NewEnumerator7`
      (`self.Build Node As Collapsing Wall` 1.0))
    (:`NewEnumerator12`
      (`self.Build Node As Wall` true 1.0))
    (:`NewEnumerator14`
      (`self.Build Node As T-Wall` 1.0))
    (:`NewEnumerator13`
      (`self.Build Node As Ladder` 1.0))))