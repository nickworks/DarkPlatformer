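; SideRoom is a procedurally generated room that builds itself from a size, offset and seed.
; Init seeds a random stream, scales the floor and usually adds two opposite side walls as BuilderWallNodes with random type, height and seed.
; It always spawns a random pickup or physics actor along the room, as the spawn-chance roll gates nothing.
; Ladder building is an empty stub.
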(fn `Build a ladder`)

(fn `Build a wall`
  (params (`Offset X` :type "Float (double-precision)") (Width :type "Float (double-precision)") (Length :type "Float (double-precision)") (Flip :type Boolean))
  (bind _random_stream (`self.Random Stream`))
  (bind _returnvalue (`AddComponent|NODE_AddWallNodeMesher-0` :`RelativeTransform` (`KismetMathLibrary.MakeTransform` (`KismetMathLibrary.MakeVector` `Offset X` (* Width 50.0 (select `bool` Flip :`false` 1.0 :`true` -1.0 :!type "Float (single-precision)"))) (struct :`Yaw` -90.0))))
  (`/Game/Blueprints/ProceduralGeneration/Builder_WallNodes.Init` _returnvalue (select `bool` (`KismetMathLibrary.RandomBoolWithWeightFromStream` 0.5 _random_stream) :`false` "NewEnumerator0" :`true` "NewEnumerator7" :!type "/Game/Blueprints/ProceduralGeneration/NodeTypes_Wall Enum") (`local.Length`) (`KismetMathLibrary.RandomFloatInRangeFromStream` 3.0 5.0 _random_stream) 0.5 (`KismetMathLibrary.RandomIntegerFromStream` 1000000 (`self.Random Stream`)) false false))

(fn `Init`
  (params (Width :type "Float (double-precision)") (Length :type "Float (double-precision)") (seed :type "Integer (by ref)") (`Offset X` :type "Float (double-precision)" :default -1.0))
  (locals (`Spawn POS` :type "Vector Structure" :default (0.0 0.0 0.0)) (`Random Offset X` :type "Float (double-precision)" :default 0.0))
  (bind _random_offset_x (`local.Random Offset X`))
  (bind _length (`local.Length`))
  (bind _width (`local.Width`))
  (set `self.room width` Width)
  (set `self.room length` Length)
  (`KismetMathLibrary.SetRandomStreamSeed` (`self.Random Stream`) seed)
  (`SceneComponent.K2_SetRelativeTransform` (`self.Floor`) (`KismetMathLibrary.MakeTransform` (`KismetMathLibrary.MakeVector` (* (+ Length `Offset X`) 50.0) 0.0 -50.0) (`KismetMathLibrary.MakeRotator` 0.0) (`KismetMathLibrary.MakeVector` (+ Length 1.0) (+ Width 1.0) 1.0)) false false)
  (`|ExecutionSequence`
    (:`then_0`
      (if (`KismetMathLibrary.RandomBoolWithWeightFromStream` 0.8 (`self.Random Stream`))
        (`self.Build a wall` _random_offset_x _width _length)
        (`self.Build a wall` _random_offset_x _width _length true)))
    (:`then_1`
      (if (`KismetMathLibrary.RandomBoolWithWeightFromStream` 0.8 (`self.Random Stream`))
        _))
    (:`then_2`
      (if (`KismetMathLibrary.RandomBoolWithWeightFromStream` 0.4 (`self.Random Stream`))
        _
        (else
          _))
      (`self.Spawn something interesting`))))

(fn `Spawn something interesting`
  (returns (`Random Stream` :type "RandomStream Structure"))
  (bind _random_stream (`self.Random Stream`))
  (`|SpawnActorFromClass` (select `int` (`KismetMathLibrary.RandomIntegerInRangeFromStream` 0 1 (`self.Random Stream`)) :`0` (select `int` (`KismetMathLibrary.RandomIntegerInRangeFromStream` 0 6 _random_stream) :`0` "/Game/Blueprints/InventoryItems/HoverBootsPickup.HoverBootsPickup_C" :`1` "/Game/Blueprints/InventoryItems/KeyPickup.KeyPickup_C" :`2` "/Game/Blueprints/InventoryItems/LightOrbsPickup.LightOrbsPickup_C" :`3` "/Game/Blueprints/InventoryItems/SanityMatrixPickup.SanityMatrixPickup_C" :`4` "/Game/Blueprints/InventoryItems/BlinkDashPickup.BlinkDashPickup_C" :`5` "/Game/Blueprints/InventoryItems/DisintegratorPickup.DisintegratorPickup_C" :`6` "/Game/Blueprints/InventoryItems/AetherVisionPickup.AetherVisionPickup_C" :!type "Actor Class Reference") :`1` (select `int` (`KismetMathLibrary.RandomIntegerInRangeFromStream` 0 2 _random_stream) :`0` "/Game/Blueprints/PhysicsLauncher.PhysicsLauncher_C" :`1` "/Game/Blueprints/PhysicsLauncher.PhysicsLauncher_C" :`2` "/Game/Blueprints/PickupablePhysicsObject.PickupablePhysicsObject_C" :!type "Actor Class Reference")) (`KismetMathLibrary.MakeTransform` (`KismetMathLibrary.TransformLocation` (`self.GetTransform`) (`KismetMathLibrary.MakeVector` (* (`self.room length`) 50.0) 0.0 50.0)) (`self.K2_GetActorRotation`)) "Undefined" "OverrideRootScale" null null)
  (return (`self.Random Stream`)))

(fn `UserConstructionScript`)