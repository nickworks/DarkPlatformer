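; Procedural dungeon room actor that builds a randomized multi-storey room with pillars, walls, floors and cross beams.
; Construction seeds its random stream from the ProceduralDungeon game mode, then rolls room height, floor count and wall segment types per side.
; BeginPlay spawns corner PillarNode actors and adds builder components for each wall segment and floor.
; Randomly sized, offset cross beams between storeys use an instanced static mesh grid.
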(event `self.ReceiveBeginPlay`
  (`self.MakePillars`)
  (`self.Make Walls And Floors`)
  (`self.Make Beams` 4))

(fn `Add Wall To Room`
  (params (`Wall Node Type` :type "/Game/Blueprints/ProceduralGeneration/NodeTypes_Wall Enum" :default "NewEnumerator0") (Location :type "Vector Structure") (Yaw :type "Float (double-precision)") (`Length of Wall` :type "Float (double-precision)") (`height of Wall` :type "Float (double-precision)") (thickness :type "Float (double-precision)") (`Is Top` :type Boolean) (`Force 100%` :type Boolean))
  (bind _returnvalue (`AddComponent|NODE_AddWallNodeMesher-2` :`RelativeTransform` (`KismetMathLibrary.MakeTransform` Location (`KismetMathLibrary.MakeRotator` 0.0 0.0 Yaw))))
  (`/Game/Blueprints/ProceduralGeneration/Builder_WallNodes.Init` _returnvalue `Wall Node Type` `Length of Wall` `height of Wall` thickness (`KismetMathLibrary.RandomIntegerFromStream` 1000000 (`self.random stream`)) `Is Top` `Force 100%`))

(fn `Generate All Data`
  (locals (`Max floors` :type Integer))
  (bind _max_floors (`local.Max Floors`))
  (set `self.Room Height` (`KismetMathLibrary.RandomFloatInRangeFromStream` 10.0 25.0 (`self.random stream`)))
  (`KismetArrayLibrary.Array_Clear` (`self.Floors`))
  (bind _output_get (set `local.Max Floors` (`KismetMathLibrary.RandomIntegerInRangeFromStream` 1 3 (`self.random stream`))))
  (for _index (range 1 (+ _output_get 1))
    (bind _wall_pieces (`self.Generate Data - One Wall` _index _max_floors))
    (bind _wall_pieces_2 (`self.Generate Data - One Wall` _index _max_floors))
    (bind _wall_pieces_3 (`self.Generate Data - One Wall` _index _max_floors))
    (bind _wall_pieces_4 (`self.Generate Data - One Wall` _index _max_floors))
    (`KismetArrayLibrary.Array_Add` (`self.Floors`) (make `/Game/Blueprints/ProceduralGeneration/FourWalls` _wall_pieces _wall_pieces_2 _wall_pieces_3 _wall_pieces_4))))

(fn `Generate Data - One Wall`
  (params (Floor :type Integer) (`Max Floor` :type Integer))
  (returns (`Wall Pieces` :type "Array of /Game/Blueprints/ProceduralGeneration/NodeTypes_Wall Enum"))
  (locals (`Array of Wall Types` :type "Array of /Game/Blueprints/ProceduralGeneration/NodeTypes_Wall Enum") (`New Wall Node` :type "/Game/Blueprints/ProceduralGeneration/NodeTypes_Wall Enum"))
  (for _index (range 1 (+ (`KismetMathLibrary.RandomIntegerInRangeFromStream` 1 4 (`self.random stream`)) 1))
    (set `local.New Wall Node` (cast `/Game/Blueprints/ProceduralGeneration/NodeTypes_Wall` (`KismetMathLibrary.Conv_IntToByte` (`KismetMathLibrary.RandomIntegerInRangeFromStream` 0 (enumcount `/Game/Blueprints/ProceduralGeneration/NodeTypes_Wall`) (`self.random stream`)))))
    (if (== _index (`local.Max Floor`))
      (if (`|EnumEquality` (`local.New Wall Node`) "NewEnumerator0")
        (set `local.New Wall Node` "NewEnumerator7")))
    (`KismetArrayLibrary.Array_Add` (`local.Array of Wall Types`) (`local.New Wall Node`)))
  (return (`local.Array of Wall Types`)))

(fn `Make a Cross Beam`
  (params (Location :type "Vector Structure") (`width X` :type "Float (double-precision)") (`width y` :type "Float (double-precision)"))
  (locals (`offset x` :type "Float (double-precision)") (`offset y` :type "Float (double-precision)") (`board x length` :type "Float (double-precision)" :default 0.0) (`board y length` :type "Float (double-precision)" :default 0.0))
  (bind _random_stream (`self.random stream`))
  (bind _returnvalue (`KismetMathLibrary.RandomFloatInRangeFromStream` 0.1 0.5 _random_stream))
  (bind _returnvalue_2 (+ _returnvalue _returnvalue))
  (bind _output_get (set `local.board x length` (* (`local.width X`) _returnvalue_2))) ; w*k
  (set `local.offset x` (* (`KismetMathLibrary.FMin` (- (/ _output_get 2.0) 0.5) (/ (- (`local.width X`) _output_get) 2.0)) 100.0 (select `bool` (`KismetMathLibrary.RandomBoolWithWeightFromStream` 0.5 _random_stream) :`false` 1.0 :`true` -1.0 :!type "Float (single-precision)")))
  (bind _output_get_2 (set `local.board y length` (* (`local.width y`) _returnvalue_2)))
  (set `local.offset y` (* (`KismetMathLibrary.FMin` (- (/ _output_get_2 2.0) 0.5) (/ (- (`local.width y`) _output_get_2) 2.0)) 100.0 (select `bool` (`KismetMathLibrary.RandomBoolWithWeightFromStream` 0.5 (`self.random stream`)) :`false` 1.0 :`true` -1.0 :!type "Float (single-precision)")))
  (`InstancedStaticMeshComponent.AddInstance` (`self.Beams - InstancedStaticMesh`) (`KismetMathLibrary.MakeTransform` (+ (`local.Location`) (`KismetMathLibrary.MakeVector` (`local.offset x`) 0.0 25.0)) (`KismetMathLibrary.MakeRotator` 0.0) (`KismetMathLibrary.MakeVector` (`local.board x length`) 1.0 0.5)))
  (`InstancedStaticMeshComponent.AddInstance` (`self.Beams - InstancedStaticMesh`) (`KismetMathLibrary.MakeTransform` (+ (`local.Location`) (`KismetMathLibrary.MakeVector` 0.0 (`local.offset y`))) (`KismetMathLibrary.MakeRotator` 0.0) (`KismetMathLibrary.MakeVector` 1.0 (`local.board y length`) 0.5))))

(fn `Make Beams`
  (params (cols :type Integer :default 4) (rows :type Integer :default 3))
  (locals (`spacing x` :type "Float (double-precision)" :default 0.0) (`min x` :type "Float (double-precision)" :default 0.0) (`spacing y` :type "Float (double-precision)" :default 0.0) (`min y` :type "Float (double-precision)" :default 0.0))
  (bind _rows (`local.rows`))
  (bind _cols (`local.cols`))
  (bind _output_get (set `local.spacing x` (* (/ (- (`self.Room Width`) 1.5) (`KismetMathLibrary.Conv_IntToDouble` _cols)) 100.0)))
  (set `local.min x` (* _output_get (/ (`KismetMathLibrary.Conv_IntToDouble` (- _cols 1)) -2.0)))
  (bind _output_get_2 (set `local.spacing y` (* (/ (- (`self.Room Length`) 1.5) (`KismetMathLibrary.Conv_IntToDouble` _rows)) 100.0)))
  (set `local.min y` (* _output_get_2 (/ (`KismetMathLibrary.Conv_IntToDouble` (- _rows 1)) -2.0)))
  (for _index (range (+ (- (`KismetArrayLibrary.Array_Length` (`self.Floors`)) 2) 1))
    (for _index_2 (range 1 (+ cols 1))
      (for _index_3 (range 1 (+ rows 1))
        (`self.Make a Cross Beam` (`KismetMathLibrary.MakeVector` (+ (* (`KismetMathLibrary.Conv_IntToDouble` (- _index_2 1)) (`local.spacing x`)) (`local.min x`)) (+ (* (`KismetMathLibrary.Conv_IntToDouble` (- _index_3 1)) (`local.spacing y`)) (`local.min y`)) (* (* (- (`self.Room Height`) 1.5) (`KismetMathLibrary.Conv_IntToDouble` (+ _index 1))) 100.0)) (/ (`local.spacing x`) 100.0) (/ (`local.spacing y`) 100.0))))))

(fn `Make Walls And Floors`
  (locals (x :type "Float (double-precision)" :default 0.0) (y :type "Float (double-precision)" :default 0.0) (`step-x` :type "Float (double-precision)" :default 0.0) (`step-y` :type "Float (double-precision)") (z :type "Float (double-precision)") (`width of node` :type "Float (double-precision)" :default 0.0) (`Is Top` :type Boolean :default false))
  (bind _floors (`self.Floors`))
  (bind _returnvalue (- (`self.Room Length`) (`self.pillar width`)))
  (bind _returnvalue_2 (- (`self.Room Width`) (`self.pillar width`)))
  (bind _returnvalue_3 (- (`self.Room Width`) (`self.pillar width`)))
  (bind _returnvalue_4 (- (`self.Room Length`) (`self.pillar width`)))
  (set `local.z` 0.0)
  (for (_array_element _array_index) _floors
    (set `local.Is Top` (== _array_index (- (`KismetArrayLibrary.Array_Length` _floors) 1)))
    (`|ExecutionSequence`
      (:`then_0`
        ;[1 1 1] North
        (set `local.x` (* _returnvalue_3 -50.0))
        (set `local.y` (* (`self.Room Length`) 50.0))
        (bind (_north _east _south _west) (break `/Game/Blueprints/ProceduralGeneration/FourWalls` _array_element))
        (bind _output_get (set `local.width of node` (/ _returnvalue_3 (`KismetMathLibrary.Conv_IntToDouble` (`KismetArrayLibrary.Array_Length` _north)))))
        (set `local.step-x` (* _output_get 100.0))
        (set `local.step-y` 0.0)
        (for _array_element_2 _north
          (`self.Add Wall To Room` _array_element_2 (`KismetMathLibrary.MakeVector` (`local.x`) (`local.y`) (`local.z`)) -90.0 (`local.width of node`) (`self.Room Height`) (`self.Wall thickness`) (`local.Is Top`))
          (set `local.x` (+ (`local.x`) (`local.step-x`)))
          (set `local.y` (+ (`local.y`) (`local.step-y`)))))
      (:`then_1`
        ;[1 1 1] East
        (set `local.x` (* (`self.Room Width`) -50.0))
        (set `local.y` (* _returnvalue_4 -50.0))
        (bind _output_get_2 (set `local.width of node` (/ _returnvalue_4 (`KismetMathLibrary.Conv_IntToDouble` (`KismetArrayLibrary.Array_Length` _east)))))
        (set `local.step-x` 0.0)
        (set `local.step-y` (* _output_get_2 100.0))
        (for _array_element_3 _east
          (`self.Add Wall To Room` _array_element_3 (`KismetMathLibrary.MakeVector` (`local.x`) (`local.y`) (`local.z`)) 0.0 (`local.width of node`) (`self.Room Height`) (`self.Wall thickness`) (`local.Is Top`))
          (set `local.x` (+ (`local.x`) (`local.step-x`)))
          (set `local.y` (+ (`local.y`) (`local.step-y`)))))
      (:`then_2`
        ;[1 1 1] South
        (set `local.x` (* _returnvalue_2 50.0))
        (set `local.y` (* (`self.Room Length`) -50.0))
        (bind _output_get_3 (set `local.width of node` (/ _returnvalue_2 (`KismetMathLibrary.Conv_IntToDouble` (`KismetArrayLibrary.Array_Length` _south)))))
        (set `local.step-x` (* _output_get_3 -100.0))
        (set `local.step-y` 0.0)
        (for _array_element_4 _south
          (`self.Add Wall To Room` _array_element_4 (`KismetMathLibrary.MakeVector` (`local.x`) (`local.y`) (`local.z`)) 90.0 (`local.width of node`) (`self.Room Height`) (`self.Wall thickness`) (`local.Is Top`))
          (set `local.x` (+ (`local.x`) (`local.step-x`)))
          (set `local.y` (+ (`local.y`) (`local.step-y`)))))
      (:`then_3`
        ;[1 1 1] West
        (set `local.x` (* (`self.Room Width`) 50.0))
        (set `local.y` (* _returnvalue 50.0))
        (bind _output_get_4 (set `local.width of node` (/ _returnvalue (`KismetMathLibrary.Conv_IntToDouble` (`KismetArrayLibrary.Array_Length` _west)))))
        (set `local.step-x` 0.0)
        (set `local.step-y` (* _output_get_4 -100.0))
        (for _array_element_5 _west
          (`self.Add Wall To Room` _array_element_5 (`KismetMathLibrary.MakeVector` (`local.x`) (`local.y`) (`local.z`)) 180.0 (`local.width of node`) (`self.Room Height`) (`self.Wall thickness`) (`local.Is Top`))
          (set `local.x` (+ (`local.x`) (`local.step-x`)))
          (set `local.y` (+ (`local.y`) (`local.step-y`)))))
      (:`then_4`
        (bind _returnvalue_5 (`AddComponent|NODE_AddBuilder_FloorNodes-0` :`RelativeTransform` (`KismetMathLibrary.MakeTransform` (`KismetMathLibrary.MakeVector` 0.0 0.0 (+ (`local.z`) -50.0)))))
        (`/Game/Blueprints/ProceduralGeneration/Builder_FloorNodes.Init` _returnvalue_5 (cast `/Game/Blueprints/ProceduralGeneration/NodeTypes_Floor` (`KismetMathLibrary.Conv_IntToByte` (`KismetMathLibrary.RandomIntegerInRangeFromStream` 0 (- (enumcount `/Game/Blueprints/ProceduralGeneration/NodeTypes_Floor`) 1) (`self.random stream`)))) (`self.Room Width`) (`self.Room Length`) (`self.random stream`) _array_index (`KismetArrayLibrary.Array_Length` (`self.Floors`))))
      (:`then_5`
        (set `local.z` (+ (`local.z`) (* (`self.Room Height`) 100.0)))))))

(fn `MakePillars`
  (locals (`Full Room Height` :type "Float (double-precision)" :default 0.0))
  (bind _returnvalue (* (`self.Room Width`) 50.0))
  (bind _returnvalue_2 (* (`self.Room Length`) 50.0))
  (bind _returnvalue_3 (* _returnvalue -1.0))
  (bind _returnvalue_4 (* _returnvalue_2 -1.0))
  (set `local.Full Room Height` (+ (* (`KismetArrayLibrary.Array_Length` (`self.Floors`)) (`self.Room Height`)) 3.0))
  (bind _returnvalue_5 (`|SpawnActorFromClass` "/Game/Blueprints/ProceduralGeneration/PillarNode.PillarNode_C" (`KismetMathLibrary.MakeTransform` (`KismetMathLibrary.TransformLocation` (`self.GetTransform`) (`KismetMathLibrary.MakeVector` _returnvalue _returnvalue_2 50.0)) (`self.K2_GetActorRotation`)) "Undefined" "OverrideRootScale" null null))
  (`/Game/Blueprints/ProceduralGeneration/PillarNode.Init` _returnvalue_5 (* (`local.Full Room Height`) (`KismetMathLibrary.RandomFloatInRangeFromStream` 1.0 1.25 (`self.random stream`))))
  (bind _returnvalue_6 (`|SpawnActorFromClass` "/Game/Blueprints/ProceduralGeneration/PillarNode.PillarNode_C" (`KismetMathLibrary.MakeTransform` (`KismetMathLibrary.TransformLocation` (`self.GetTransform`) (`KismetMathLibrary.MakeVector` _returnvalue _returnvalue_4 50.0)) (`self.K2_GetActorRotation`)) "Undefined" "OverrideRootScale" null null))
  (`/Game/Blueprints/ProceduralGeneration/PillarNode.Init` _returnvalue_6 (* (`local.Full Room Height`) (`KismetMathLibrary.RandomFloatInRangeFromStream` 1.0 1.25 (`self.random stream`))))
  (bind _returnvalue_7 (`|SpawnActorFromClass` "/Game/Blueprints/ProceduralGeneration/PillarNode.PillarNode_C" (`KismetMathLibrary.MakeTransform` (`KismetMathLibrary.TransformLocation` (`self.GetTransform`) (`KismetMathLibrary.MakeVector` _returnvalue_3 _returnvalue_4 50.0)) (`self.K2_GetActorRotation`)) "Undefined" "OverrideRootScale" null null))
  (`/Game/Blueprints/ProceduralGeneration/PillarNode.Init` _returnvalue_7 (* (`local.Full Room Height`) (`KismetMathLibrary.RandomFloatInRangeFromStream` 1.0 1.25 (`self.random stream`))))
  (bind _returnvalue_8 (`|SpawnActorFromClass` "/Game/Blueprints/ProceduralGeneration/PillarNode.PillarNode_C" (`KismetMathLibrary.MakeTransform` (`KismetMathLibrary.TransformLocation` (`self.GetTransform`) (`KismetMathLibrary.MakeVector` _returnvalue_3 _returnvalue_2 50.0)) (`self.K2_GetActorRotation`)) "Undefined" "OverrideRootScale" null null))
  (`/Game/Blueprints/ProceduralGeneration/PillarNode.Init` _returnvalue_8 (* (`local.Full Room Height`) (`KismetMathLibrary.RandomFloatInRangeFromStream` 1.0 1.25 (`self.random stream`)))))

(fn `Setup random seed`
  (locals (Seed :type Integer :default 0))
  (bind _asprocedural_dungeon (cast `/Game/Blueprints/PlayerCharacter/ProceduralDungeon` (`GameplayStatics.GetGameMode`)))
  (bind _output_get (set `local.Seed` (`KismetMathLibrary.RandomIntegerFromStream` 1000000 (`/Game/Blueprints/PlayerCharacter/ProceduralDungeon.random stream` _asprocedural_dungeon))))
  (`KismetMathLibrary.SetRandomStreamSeed` (`self.random stream`) _output_get))

(fn `UserConstructionScript`
  (`self.Setup random seed`)
  (`self.Generate All Data`))