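; Game instance that handles warping between the Manor and the procedural maze Aether, plus shared random loot spawning.
; LoadLevel swaps streamed levels behind a loader widget, destroying the player and respawning it at a PlayerStart once the fade signals back.
; Entering the Aether caches held relics and reseeds the random stream; dying clears that loadout.
; Spawn helpers use that stream to pick loot or alternatives like Mimics.
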(event `Warp To`
  (params (Destination :type "/Game/Blueprints/WarpGateDestination Enum" :default "NewEnumerator0"))
  ;[1 1 1] Stream in a Level (must be in Loader scene to work)
  (switch `/Game/Blueprints/WarpGateDestination` Destination
    (:`NewEnumerator0`
      (`self.Warp to Manor (Died)`))
    (:`NewEnumerator1`
      (`self.Warp to Aether`))))

(event `Warp to Manor (Died)`
  ;[1 1 1] Stream in a Level (must be in Loader scene to work)
  (set `self.isInTheAether` false)
  (`KismetArrayLibrary.Array_Clear` (`self.Item Loadout`))
  (`self.Load Level` "Manor2"))

(event `Warp to Aether`
  ;[1 1 1] Stream in a Level (must be in Loader scene to work)
  (set `self.isInTheAether` true)
  (`self.Cache Players Inventory`)
  (`self.Load Level` "ProceduralMAZE")
  (`KismetMathLibrary.SetRandomStreamSeed` (`self.random stream`) (`KismetMathLibrary.RandomInteger` 1000000)))

(event `Load Level`
  (params (`next level` :type Name))
  (bind _player_ref (`self.player ref`))
  ;[1 1 1] Stream in a Level (must be in Loader scene to work)
  (if (`self.isLoading`)
    _
    (elif (not (== `next level` (`self.Current Level Name`)))
      (set `self.isLoading` true)
      (bind _returnvalue (`|CreateWidget` "/Game/Blueprints/GUI/LoaderGUI.LoaderGUI_C"))
      (`UserWidget.AddToPlayerScreen` _returnvalue 1000)
      (add `/Game/Blueprints/GUI/LoaderGUI.FadingOut` _returnvalue (delegate `Fading Back`))
      (`/Game/Blueprints/GUI/LoaderGUI.Begin "Loading"` _returnvalue (!= (`self.Current Level Name`) "None"))
      (`KismetSystemLibrary.Delay` 1.0)
      (`/Engine/EditorBlueprintResources/StandardMacros.IsValid` _player_ref
        (:`Is Valid`
          (`Actor.K2_DestroyActor` _player_ref))
        (:`Is Not Valid`
          _))
      (`GameplayStatics.UnloadStreamLevel` (`self.Current Level Name`))
      (bind _output_get (set `self.Current Level Name` `next level`))
      (`GameplayStatics.LoadStreamLevel` _output_get true))))

(event `Fading Back`
  ;[1 1 1] Stream in a Level (must be in Loader scene to work)
  (`self.Spawn Player`)
  (`KismetSystemLibrary.Delay` 0.4)
  (set `self.isLoading` false)
  (`GameplayStatics.PlaySound2D` "/Game/Audio/Spawn.Spawn" 1.0 1.0 0.0 null null))

(event `Spawn Player At Start`
  (bind _returnvalue (`GameplayStatics.GetActorOfClass` "/Script/Engine.PlayerStart"))
  (`/Engine/EditorBlueprintResources/StandardMacros.IsValid` _returnvalue
    (:`Is Valid`
      (bind (_returnvalue_location _returnvalue_rotation) (`KismetMathLibrary.BreakTransform` (`Actor.GetTransform` _returnvalue)))
      (bind _returnvalue_2 (`|SpawnActorFromClass` "/Game/Blueprints/PlayerCharacter/PlayerCharacter.PlayerCharacter_C" (`KismetMathLibrary.MakeTransform` _returnvalue_location _returnvalue_rotation) "Undefined" "OverrideRootScale" _returnvalue null))
      (`Controller.Possess` (`GameplayStatics.GetPlayerController` 0) _returnvalue_2))
    (:`Is Not Valid`
      (`KismetSystemLibrary.PrintString` "No PlayerStart found in level"))))

(event `Cache Players Inventory`
  (bind _player_ref (`self.Player Ref`))
  (`/Engine/EditorBlueprintResources/StandardMacros.IsValid` _player_ref
    (:`Is Valid`
      (`KismetArrayLibrary.Array_Clear` (`self.Item Loadout`))
      (for _array_element (`/Game/Blueprints/PlayerCharacter/InventorySystem.Held Relics` (`/Game/Blueprints/PlayerCharacter/PlayerCharacter.InventorySystem` _player_ref))
        (`KismetArrayLibrary.Array_Add` (`self.Item Loadout`) (make `/Game/Blueprints/InventoryItems/ItemLoadout` (`GameplayStatics.GetObjectClass` _array_element) (`/Game/Blueprints/InventoryItems/ItemAbilities/_ItemAbility.Amount in this stack` _array_element)))))))

(fn `Spawn Loot At`
  (params (SpawnTransform :type "Transform Structure") (Owner :type "Actor Object Reference"))
  (`|SpawnActorFromClass` (select `int` (`KismetMathLibrary.RandomIntegerInRangeFromStream` 0 9 (`self.Random Stream`)) :`0` "/Game/Blueprints/InventoryItems/ItemAbilities/AetherVision.AetherVision_C" :`1` "/Game/Blueprints/InventoryItems/ItemAbilities/AncientKey.AncientKey_C" :`2` "/Game/Blueprints/InventoryItems/ItemAbilities/AntiGravityBrew.AntiGravityBrew_C" :`3` "/Game/Blueprints/InventoryItems/ItemAbilities/BlinkDash.BlinkDash_C" :`4` "/Game/Blueprints/InventoryItems/ItemAbilities/Disintegrator.Disintegrator_C" :`5` "/Game/Blueprints/InventoryItems/ItemAbilities/FrequencyAttuner.FrequencyAttuner_C" :`6` "/Game/Blueprints/InventoryItems/ItemAbilities/HoverBoots.HoverBoots_C" :`7` "/Game/Blueprints/InventoryItems/ItemAbilities/LightOrb.LightOrb_C" :`8` "/Game/Blueprints/InventoryItems/ItemAbilities/SanityMatrix.SanityMatrix_C" :`9` "/Game/Blueprints/InventoryItems/ItemAbilities/TentacleFlesh.TentacleFlesh_C" :!type "Actor Class Reference") SpawnTransform "Undefined" "OverrideRootScale" Owner null))

(fn `Spawn Loot or Something Else`
  (params (`Weight for Loot` :type "Float (double-precision)" :default 0.5) (SpawnTransform :type "Transform Structure") (Owner :type "Actor Object Reference"))
  (if (`KismetMathLibrary.RandomBoolWithWeightFromStream` `Weight for Loot` (`self.random stream`))
    (`self.Spawn Loot At` SpawnTransform Owner)
    (else
      (`|SpawnActorFromClass` (select `int` (`KismetMathLibrary.RandomIntegerInRangeFromStream` 0 3 (`self.Random Stream`)) :`0` "/Game/Blueprints/PhysicsLauncher.PhysicsLauncher_C" :`1` "/Game/Blueprints/PhysicsLauncher.PhysicsLauncher_C" :`2` "/Game/Blueprints/Mimic/Mimic.Mimic_C" :`3` "/Game/Blueprints/InventoryItems/ItemAbilities/SanityMatrix.SanityMatrix_C" :`4` null :!type "Actor Class Reference") SpawnTransform "Undefined" "OverrideRootScale" Owner null))))

(fn `Spawn Player`
  (bind _returnvalue (`GameplayStatics.GetActorOfClass` "/Script/Engine.PlayerStart"))
  (`/Engine/EditorBlueprintResources/StandardMacros.IsValid` _returnvalue
    (:`Is Valid`
      (bind (_returnvalue_location _returnvalue_rotation) (`KismetMathLibrary.BreakTransform` (`Actor.GetTransform` _returnvalue)))
      (bind _returnvalue_2 (`|SpawnActorFromClass` "/Game/Blueprints/PlayerCharacter/PlayerCharacter.PlayerCharacter_C" (`KismetMathLibrary.MakeTransform` _returnvalue_location _returnvalue_rotation) "Undefined" "OverrideRootScale" _returnvalue null))
      (`Controller.Possess` (`GameplayStatics.GetPlayerController` 0) _returnvalue_2)
      (set `self.Player Ref` _returnvalue_2))
    (:`Is Not Valid`
      (`KismetSystemLibrary.PrintString` "No PlayerStart found in level"))))