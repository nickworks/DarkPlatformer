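; Level-generation actor that builds a procedural maze dungeon on BeginPlay and reloads the ProceduralMAZE level shortly after the player dies.
; BuildDungeon spawns a centred grid of Room actors with jittered position and rotation, leaving the origin cell empty as home base.
; BuildGroundZero then spawns a GroundZero actor.
; A shared random stream drives region size and jitter and hands each spawned piece its own seed.
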(event `self.ReceiveBeginPlay`
  (bind _returnvalue (`KismetMathLibrary.RandomFloatInRangeFromStream` 3800.0 4000.0 (`self.random stream`)))
  (`self.Build Dungeon` 5 5 _returnvalue _returnvalue)
  (`self.Build Ground Zero`))

(event `On Player Dead`
  (`KismetSystemLibrary.Delay` 2.0)
  (`GameplayStatics.OpenLevel` "ProceduralMAZE"))

(fn `Build Dungeon`
  (params (Rows :type Integer :default 3) (Columns :type Integer :default 3) (`Region size x` :type "Float (double-precision)" :default 5500.0) (`Region size y` :type "Float (double-precision)" :default 5500.0))
  (locals (`Offset X` :type "Float (double-precision)") (`Offset Y` :type "Float (double-precision)"))
  (bind _random_stream (`self.random stream`))
  (bind _returnvalue (/ (- Columns 1) -2))
  (bind _returnvalue_2 (`KismetMathLibrary.RandomFloatInRangeFromStream` -2.0 2.0 _random_stream))
  (bind _returnvalue_3 (`KismetMathLibrary.RandomFloatInRangeFromStream` -1.0 1.0 _random_stream))
  (bind _returnvalue_4 (/ (- Rows 1) -2))
  (bind _returnvalue_5 (+ _returnvalue_3 _returnvalue_3))
  (set `self.REGION WIDTH` `Region size x`)
  (set `self.REGION LENGTH` `Region size y`)
  (for _index (range _returnvalue_4 (+ (+ _returnvalue_4 (`local.Rows`) -1) 1))
    (for _index_2 (range _returnvalue (+ (+ _returnvalue (`local.Columns`) -1) 1))
      (if (not (and (== _index_2 0) (== _index 0)))
        (bind _returnvalue_6 (`|SpawnActorFromClass` "/Game/Blueprints/ProceduralGeneration/Room.Room_C" (`KismetMathLibrary.MakeTransform` (`KismetMathLibrary.MakeVector` (+ (+ (* _index (`self.REGION WIDTH`)) 0.0) (`KismetMathLibrary.RandomFloatInRangeFromStream` -100.0 100.0 (`self.random stream`))) (+ (+ (* _index_2 (`self.REGION LENGTH`)) 0.0) (`KismetMathLibrary.RandomFloatInRangeFromStream` -100.0 100.0 (`self.random stream`))) (`KismetMathLibrary.RandomFloatInRangeFromStream` -100.0 100.0 (`self.random stream`))) (`KismetMathLibrary.MakeRotator` _returnvalue_5 _returnvalue_5 (+ _returnvalue_2 _returnvalue_2))) "Undefined" "OverrideRootScale" null null))
        (`/Game/Blueprints/ProceduralGeneration/Room.Init From Seed` _returnvalue_6 (`KismetMathLibrary.RandomIntegerFromStream` 12000000 (`self.random stream`)))))))

(fn `Build Ground Zero`
  (locals (scale :type "Float (double-precision)" :default 0.0))
  (bind _returnvalue (`|SpawnActorFromClass` "/Game/Blueprints/ProceduralGeneration/GroundZero.GroundZero_C" (`KismetMathLibrary.MakeTransform` (0.0 0.0 0.0)) "Undefined" "OverrideRootScale" null null))
  (`/Game/Blueprints/ProceduralGeneration/GroundZero.Init` _returnvalue (`KismetMathLibrary.RandomIntegerFromStream` 1000000 (`self.random stream`))))

(fn `UserConstructionScript`)