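; Inventory component for the first-person character that holds stackable relics, lets the player cycle through and use them, and creates the HUD that displays them.
; Each relic type is one spawned actor with a stack count, seeded from a starting list.
; A successful use decrements consumables and charges the relic's sanity cost as damage to the player.
; Relics can also be removed by type, optionally applying that cost, and changes refresh the HUD.
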(event `self.ReceiveBeginPlay`
  (bind _asfirst_person_character (cast `/Game/Blueprints/PlayerCharacter/FirstPersonCharacter` (`self.GetOwner`)))
  (set `self.Player` _asfirst_person_character)
  (bind _returnvalue (`|CreateWidget` "/Game/Blueprints/Widgets/Hud.Hud_C"))
  (bind _output_get (set `self.The HUD` _returnvalue))
  (`UserWidget.AddToPlayerScreen` _output_get 0)
  (for _array_element (`self.Starting Relics`)
    (`self.Add Relic` _array_element))
  (`self.Update the GUI`))

(event `Next Item`
  (bind _returnvalue (+ (`self.Current relic`) 1))
  (set `self.Current relic` (select `bool` (>= _returnvalue (`KismetArrayLibrary.Array_Length` (`self.Held Relics`))) :`false` _returnvalue))
  (if (> (`KismetArrayLibrary.Array_Length` (`self.Held Relics`)) 0) :!label _label
    (`self.Update the GUI`)))

(event `Prev Item`
  (bind _returnvalue (- (`self.Current relic`) 1))
  (set `self.Current relic` (select `bool` (< _returnvalue 0) :`false` _returnvalue :`true` (- (`KismetArrayLibrary.Array_Length` (`self.Held Relics`)) 1)))
  (goto _label))

(event `Use Relic`
  (`self.Use Item At Index` (`self.Current relic`))
  (`self.Update the GUI`))

(fn `Add Relic`
  (params (`Relic Type` :type "/Game/Blueprints/InventoryItems/ItemAbilities/_Ability Class Reference") (Quantity :type Integer :default 1))
  (locals (`add new stack` :type Boolean))
  (set `local.add new stack` true)
  (for _array_element (`self.Held Relics`)
    (if (== `Relic Type` (`GameplayStatics.GetObjectClass` _array_element))
      (set `local.add new stack` false)
      (set `/Game/Blueprints/InventoryItems/ItemAbilities/_Ability.Amount in this stack` (+ (`/Game/Blueprints/InventoryItems/ItemAbilities/_Ability.Amount in this stack` _array_element) (`local.Quantity`)) _array_element)
      (break)))
  (if (`local.add new stack`)
    (bind _returnvalue (`|SpawnActorFromClass` `Relic Type` (`KismetMathLibrary.MakeTransform` (0.0 0.0 0.0)) "Undefined" "OverrideRootScale" null null))
    (set `/Game/Blueprints/InventoryItems/ItemAbilities/_Ability.Amount in this stack` (`local.Quantity`) _returnvalue)
    (`KismetArrayLibrary.Array_Add` (`self.Held Relics`) _returnvalue)
    (`self.Update the GUI`)
    (else
      (`self.Update the GUI`))))

(fn `Relic affects player's sanity`
  (params (Relic :type "/Game/Blueprints/InventoryItems/ItemAbilities/_Ability Object Reference"))
  (`GameplayStatics.ApplyDamage` (`self.Player`) (`/Game/Blueprints/InventoryItems/ItemAbilities/_Ability.Sanity Cost` Relic)))

(fn `Remove item at index`
  (params (Index :type Integer) (Amount :type Integer :default 1))
  (locals (`the removed relic` :type "/Game/Blueprints/InventoryItems/ItemAbilities/_Ability Object Reference"))
  (bind _the_removed_relic (`local.the removed relic`))
  (bind _current_relic (`self.Current relic`))
  (bind _output_get (set `local.the removed relic` (`|GetArrayItem` (`self.Held Relics`) Index)))
  (`/Engine/EditorBlueprintResources/StandardMacros.IsValid` _output_get
    (:`Is Valid`
      (if (`/Game/Blueprints/InventoryItems/ItemAbilities/_Ability.Is consumable?` _the_removed_relic)
        (bind _output_get_2 (set `/Game/Blueprints/InventoryItems/ItemAbilities/_Ability.Amount in this stack` (- (`/Game/Blueprints/InventoryItems/ItemAbilities/_Ability.Amount in this stack` _the_removed_relic) Amount) _the_removed_relic))
        (if (<= _output_get_2 0)
          (`KismetArrayLibrary.Array_Remove` (`self.Held Relics`) (`local.index`))
          (if (<= (`local.index`) _current_relic)
            (set `self.Current relic` (`KismetMathLibrary.Max` (- _current_relic 1)))))))
    (:`Is Not Valid`
      (`KismetSystemLibrary.PrintString` "invalid item index?"))))

(fn `Remove Item If Held`
  (params (Type :type "/Game/Blueprints/InventoryItems/ItemAbilities/_Ability Class Reference") (Amount :type Integer :default 1) (`And Apply Damage?` :type Boolean))
  (returns (`Removed any?` :type Boolean))
  (for (_array_element _array_index) (`self.Held Relics`)
    (if (== Type (`GameplayStatics.GetObjectClass` _array_element))
      (if (`local.And Apply Damage?`)
        (`self.Relic affects player's sanity` _array_element))
      (`self.Remove item at index` _array_index (`local.Amount`))
      (`self.Update the GUI`)
      (return true)))
  (return false))

(fn `Update the GUI`
  (bind _the_hud (`self.The HUD`))
  (`/Engine/EditorBlueprintResources/StandardMacros.IsValid` _the_hud
    (:`Is Valid`
      (`/Game/Blueprints/Widgets/Hud.UpdateGUI` _the_hud self))))

(fn `Use Item At Index`
  (params (index :type Integer))
  (locals (`the used relic` :type "/Game/Blueprints/InventoryItems/ItemAbilities/_Ability Object Reference"))
  (bind _output_get (set `local.the used relic` (`|GetArrayItem` (`self.Held Relics`) index)))
  (`/Engine/EditorBlueprintResources/StandardMacros.IsValid` _output_get
    (:`Is Valid`
      (bind _success_ (`/Game/Blueprints/InventoryItems/ItemAbilities/_Ability.Use Relic` (`local.the used relic`) (`self.Player`)))
      (if _success_
        (`self.Remove item at index` (`local.index`))
        (`self.Relic affects player's sanity` (`local.the used relic`))))))