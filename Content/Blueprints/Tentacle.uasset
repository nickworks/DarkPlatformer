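; Tentacle Blueprint that procedurally builds a curled, tapering chain of instanced static mesh segments in its Construction Script.
; Each segment composes a fixed upward offset, rotation and slight shrink onto the previous transform, so the bend and taper accumulate along the length.
; The twist is rolled once from a randomly reseeded stream, giving a uniform curl that changes whenever the script reruns.
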(fn `UserConstructionScript`
  (locals (rot :type "Rotator Structure" :default (struct)) (xform :type "Transform Structure"))
  (bind _xform (`local.xform`))
  (bind _random_stream (`self.random stream`))
  (bind _returnvalue (`KismetMathLibrary.RandomFloatInRangeFromStream` -15.0 15.0 _random_stream))
  (`KismetMathLibrary.SetRandomStreamSeed` (`self.random stream`) (`KismetMathLibrary.RandomInteger` 8000000))
  (set `local.rot` (`KismetMathLibrary.MakeRotator` _returnvalue _returnvalue (`KismetMathLibrary.RandomFloatInRangeFromStream` -20.0 20.0 _random_stream)))
  (set `local.xform` (`KismetMathLibrary.MakeTransform` (0.0 0.0 0.0) (struct) (2.0 2.0 2.0)))
  (for _ (range 1 18)
    (`InstancedStaticMeshComponent.AddInstance` (`self.InstancedStaticMesh`) _xform)
    (set `local.xform` (`KismetMathLibrary.ComposeTransforms` (`KismetMathLibrary.MakeTransform` (* (`KismetMathLibrary.Vector_Up`) 120.0) (`local.rot`) (0.96 0.96 0.98)) _xform))))