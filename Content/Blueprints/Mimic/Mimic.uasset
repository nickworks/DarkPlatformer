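; Mimic is a flying enemy pawn that poses as a chamfered cube until PawnSensing spots the first-person character.
; TurnOnOrOff then swaps the cube for a sphere and point light and starts channeling.
; While channeling, Tick deals radial damage around the Mimic and applies capsule force toward the player.
; Seeing another pawn restores the disguise, while an invalid player only clears the channeling flag.
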(event `self.ReceiveBeginPlay`
  (`CharacterMovementComponent.SetMovementMode` (`self.CharacterMovement`) "MOVE_Flying" 0))

(event `self.ReceiveTick`
  (params (DeltaSeconds :type "Float (single-precision)"))
  (bind _capsulecomponent (`self.CapsuleComponent`))
  (if (`self.IsChanneling`)
    (`/Engine/EditorBlueprintResources/StandardMacros.IsValid` (`self.player`)
      (:`Is Valid`
        (`GameplayStatics.ApplyRadialDamage` :`BaseDamage` 2.0 :`Origin` (`self.K2_GetActorLocation`) :`DamageRadius` 700.0 :`DamageCauser` self :`InstigatedByController` null)
        (`PrimitiveComponent.AddForce` _capsulecomponent (* (`KismetMathLibrary.Normal` (- (`self.K2_GetActorLocation` (`self.player`)) (`SceneComponent.K2_GetComponentLocation` _capsulecomponent))) 1000000.0) "None" false))
      (:`Is Not Valid`
        (set `self.IsChanneling` false)))))

(event `self.PawnSensing.OnSeePawn`
  (params (Pawn :type "Pawn Object Reference"))
  (bind _asfirst_person_character (cast `/Game/Blueprints/PlayerCharacter/FirstPersonCharacter` Pawn)
    (:`then`
      (set `self.player` _asfirst_person_character)
      (`self.Turn On or Off` true))
    (:`CastFailed`
      (`self.Turn On or Off` false))))

(fn `Turn On or Off`
  (params (`Is On?` :type Boolean))
  (if (!= (`self.IsChanneling`) `Is On?`)
    (bind _output_get (set `self.IsChanneling` `Is On?`))
    (`SceneComponent.SetHiddenInGame` (`self.1M_Cube_Chamfer`) _output_get false)
    (`SceneComponent.SetHiddenInGame` (`self.Sphere`) (not (`self.IsChanneling`)) false)
    (`SceneComponent.SetHiddenInGame` (`self.PointLight`) (not (`self.IsChanneling`)) false)))

(fn `UserConstructionScript`)