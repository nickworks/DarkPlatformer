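; SideRoom is a room piece with a floor and two long side walls, sized at runtime from a width and length.
; Init stretches the Floor one unit beyond each dimension and shifts it forward by half the length, so the room extends from the actor's origin.
; It then adds two rotated WallNodeMesher components at plus and minus half the width, each initialized to the room's length, with no end walls.
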(fn `Init`
  (params (Width :type "Float (double-precision)") (Length :type "Float (double-precision)"))
  (`SceneComponent.K2_SetRelativeTransform` (`self.Floor`) (`KismetMathLibrary.MakeTransform` (`KismetMathLibrary.MakeVector` (* Length 50.0)) (struct) (`KismetMathLibrary.MakeVector` (+ Length 1.0) (+ Width 1.0) 1.0)) false false)
  ;[1 1 1] Right Wall
  (bind _returnvalue (`AddComponent|NODE_AddWallNodeMesher-0` :`RelativeTransform` (`KismetMathLibrary.MakeTransform` (`KismetMathLibrary.MakeVector` 0.0 (* (`local.Width`) 50.0)) (struct :`Yaw` -90.0) (1.0 1.0 1.0))))
  (`/Game/Blueprints/WallNodeMesher.Init` _returnvalue "NewEnumerator0" (`local.Length`) 4.0 0.5 (0.0 0.0 0.0))
  ;[1 1 1] Left Wall
  (bind _returnvalue_2 (`AddComponent|NODE_AddWallNodeMesher-1` :`RelativeTransform` (`KismetMathLibrary.MakeTransform` (`KismetMathLibrary.MakeVector` 0.0 (* (`local.Width`) -50.0)) (struct :`Yaw` -90.0))))
  (`/Game/Blueprints/WallNodeMesher.Init` _returnvalue_2 "NewEnumerator0" (`local.Length`) 4.0 0.5 (0.0 0.0 0.0)))

(fn `UserConstructionScript`)