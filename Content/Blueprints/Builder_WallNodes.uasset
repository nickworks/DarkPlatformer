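; Procedural wall-section builder that creates a plain, crumbling or torch-lit wall, or a passage, from a node type, dimensions and seed.
; Block fill adds jittered mesh instances in rows and columns with occasional gaps, all driven by one seeded random stream.
; Crumbling fill narrows each row from both sides.
; Passages frame an opening under a solid or crumbling top, optionally spawn a lockable door, and always spawn a seeded SideRoom.
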(fn `Build Section As Collapsing Wall`
  (`self.Fill Region With Crumbling Blocks` (* (`self.thickness`) 100.0) (* (`self.width`) 100.0) (* (`self.height`) 100.0)))

(fn `Build Section As Passageway`
  (params (`Passage Width` :type "Float (double-precision)") (`Passage Height` :type "Float (double-precision)") (`Has Door` :type Boolean) (`Is Locked` :type Boolean) (`Flip inside / outside` :type Boolean))
  (locals (`Door Location` :type "Vector Structure" :default (0.0 0.0 0.0)) (`Door Rotation` :type "Rotator Structure" :default (struct)))
  (bind _random_stream (`self.Random Stream`))
  (bind _passage_height (`local.Passage Height`))
  (bind (_door_rotation_roll _door_rotation_pitch _door_rotation_yaw) (`KismetMathLibrary.BreakRotator` (`local.Door Rotation`)))
  (bind _returnvalue (`KismetMathLibrary.RandomFloatInRangeFromStream` 0.2 0.8 (`self.Random Stream`)))
  (bind _returnvalue_2 (* (`local.Passage Height`) 100.0))
  (bind _returnvalue_3 (* (`self.thickness`) 100.0))
  (bind _returnvalue_4 (* (`self.thickness`) 100.0))
  (bind _returnvalue_5 (* (`self.width`) 100.0))
  (bind _returnvalue_6 (* _passage_height 100.0))
  (bind _returnvalue_7 (/ (- (`self.width`) (`local.Passage Width`)) 2.0))
  (bind _returnvalue_8 (* (- (`self.height`) _passage_height) 100.0))
  (bind _returnvalue_9 (* _returnvalue_7 100.0))
  (`self.Fill Region With Blocks` _returnvalue_3 _returnvalue_9 _returnvalue_2) ; Region Left of Door
  (`self.Fill Region With Blocks` _returnvalue_3 _returnvalue_9 _returnvalue_2 (* (+ _returnvalue_7 (`local.Passage Width`)) 100.0)) ; Region Right of Door
  (if (`KismetMathLibrary.RandomBoolWithWeightFromStream` 0.5 (`self.Random Stream`))
    (`self.Fill Region With Blocks` _returnvalue_4 _returnvalue_5 _returnvalue_8 0.0 _returnvalue_6) ; Region Above Door
    (else
      (`self.Fill Region With Crumbling Blocks` _returnvalue_4 _returnvalue_5 _returnvalue_8 0.0 _returnvalue_6)))
  (bind (_location_ws _rotation_ws) (`self.Get Door Position` (0.0 0.0 0.0) (`local.Flip inside / outside`)))
  (set `local.Door Location` _location_ws)
  (set `local.Door Rotation` _rotation_ws)
  ;[1 1 1] Make Door
  (if (`local.Has Door`)
    (bind _returnvalue_10 (`|SpawnActorFromClass` "/Game/Blueprints/DoorBp.DoorBp_C" (`KismetMathLibrary.MakeTransform` (`local.Door Location`) (`local.Door Rotation`)) "Undefined" "OverrideRootScale" null null))
    (`/Game/Blueprints/DoorBp.Init` _returnvalue_10 (`local.Passage Width`) (`local.Passage Height`) (`local.Is Locked`)))
  ;[1 1 1] Make Side Room
  (bind _returnvalue_11 (`|SpawnActorFromClass` "/Game/Blueprints/SideRoom.SideRoom_C" (`KismetMathLibrary.MakeTransform` (+ (`local.Door Location`) (0.0 0.0 0.0)) (`KismetMathLibrary.MakeRotator` (* _door_rotation_roll _returnvalue) (* _door_rotation_pitch _returnvalue) _door_rotation_yaw)) "Undefined" "OverrideRootScale" null null))
  (`/Game/Blueprints/SideRoom.Init` _returnvalue_11 (`KismetMathLibrary.RandomFloatInRangeFromStream` 4.0 6.0 _random_stream) (`KismetMathLibrary.RandomFloatInRangeFromStream` 4.0 16.0 _random_stream) (`KismetMathLibrary.RandomIntegerFromStream` 1000000 _random_stream)))

(fn `Build Section As Wall`
  (`self.Fill Region With Blocks` (* (`self.thickness`) 100.0) (* (`self.width`) 100.0) (* (`self.height`) 100.0)))

(fn `Fill Region With Blocks`
  (params (`Region Thickness` :type "Float (double-precision)") (`Region Width` :type "Float (double-precision)") (`Region Height` :type "Float (double-precision)") (`Y Min` :type "Float (double-precision)") (`Z Min` :type "Float (double-precision)"))
  (locals (`Block width` :type "Float (double-precision)" :default 0.0) (`Block height` :type "Float (double-precision)" :default 0.0) (`Columns of blocks` :type Integer :default 0) (`Rows of blocks` :type Integer :default 0) (Y :type "Float (double-precision)") (Z :type "Float (double-precision)"))
  (bind _random_stream (`self.Random Stream`))
  (bind _returnvalue (`KismetMathLibrary.RandomFloatInRangeFromStream` -0.5 0.5 (`self.Random Stream`)))
  (bind _returnvalue_2 (`KismetMathLibrary.RandomFloatInRangeFromStream` -2.0 2.0 (`self.Random Stream`)))
  (bind _output_get (set `local.Columns of blocks` (`KismetMathLibrary.FTrunc` (/ (`local.Region Width`) (`self.target block width`)))))
  (set `local.Block width` (/ (`local.Region Width`) (`KismetMathLibrary.Conv_IntToDouble` _output_get)))
  (bind _output_get_2 (set `local.Rows of blocks` (`KismetMathLibrary.FTrunc` (/ (`local.Region Height`) (`self.target block height`)))))
  (set `local.Block height` (/ (`local.Region Height`) (`KismetMathLibrary.Conv_IntToDouble` _output_get_2)))
  (set `local.Y` (+ (`local.Y Min`) (/ (`local.Block width`) -2.0)))
  (set `local.Z` (+ (`local.Z Min`) (/ (`local.Block height`) 2.0)))
  (for _ (range 1 (+ (`local.Rows of blocks`) 1))
    (for _ (range 1 (+ (`local.Columns of blocks`) 1))
      (set `local.Y` (+ (`local.Y`) (`local.Block width`)))
      (if (`KismetMathLibrary.RandomBoolWithWeightFromStream` 0.95 _random_stream)
        (`self.AddInstance` (`KismetMathLibrary.MakeTransform` (`KismetMathLibrary.MakeVector` (`KismetMathLibrary.RandomFloatInRangeFromStream` 0.0 20.0 _random_stream) (`local.Y`) (`local.Z`)) (`KismetMathLibrary.MakeRotator` 0.0 (+ _returnvalue _returnvalue _returnvalue _returnvalue) (+ _returnvalue_2 _returnvalue_2 _returnvalue_2 _returnvalue_2)) (`KismetMathLibrary.MakeVector` (* (`self.thickness`) (`KismetMathLibrary.RandomFloatInRangeFromStream` 1.0 2.0 (`self.Random Stream`))) (/ (`local.Block width`) 100.0) (/ (`local.Block height`) 100.0))))))
    (set `local.Z` (+ (`local.Z`) (`local.Block height`)))
    (set `local.Y` (+ (`local.Y Min`) (/ (`local.Block width`) -2.0)))))

(fn `Fill Region With Crumbling Blocks`
  (params (`Region Thickness` :type "Float (double-precision)") (`Region Width` :type "Float (double-precision)") (`Region Height` :type "Float (double-precision)") (`Y Min` :type "Float (double-precision)") (`Z Min` :type "Float (double-precision)"))
  (locals (`Percent Remaining on Left` :type "Float (double-precision)") (`Percent Remaining on Right` :type "Float (double-precision)") (`Stacks of blocks` :type Integer :default 0))
  (bind _target_block_height (`self.target block height`))
  (bind _target_block_height_2 (`self.target block height`))
  (bind _returnvalue (`KismetMathLibrary.RandomFloatInRangeFromStream` 0.25 0.5 (`self.Random Stream`)))
  (bind _returnvalue_2 (`KismetMathLibrary.RandomFloatInRangeFromStream` 0.75 0.9 (`self.Random Stream`)))
  (bind _returnvalue_3 (* (`local.Region Width`) (`local.Percent Remaining on Right`)))
  (bind _returnvalue_4 (`KismetMathLibrary.FTrunc` (/ `Region Height` (`self.target block height`))))
  (set `local.Percent Remaining on Left` _returnvalue)
  (set `local.Percent Remaining on Right` _returnvalue)
  (set `local.Stacks of blocks` _returnvalue_4)
  (for _index (range (+ _returnvalue_4 1))
    (`self.Fill Region With Blocks` (`local.Region Thickness`) (* (`local.Region Width`) (`local.Percent Remaining on Left`)) _target_block_height 0.0 (* _index _target_block_height))
    (`self.Fill Region With Blocks` (`local.Region Thickness`) _returnvalue_3 _target_block_height_2 (- (`local.Region Width`) _returnvalue_3) (* _index _target_block_height_2))
    (set `local.Percent Remaining on Left` (* _returnvalue_2 (`local.Percent Remaining on Left`)))
    (set `local.Percent Remaining on Right` (* _returnvalue_2 (`local.Percent Remaining on Right`)))))

(fn `Get Door Position`
  (params (`Direction outward` :type "Vector Structure") (Flip :type Boolean))
  (returns (`Location WS` :type "Vector Structure") (`Rotation WS` :type "Rotator Structure"))
  (return (`KismetMathLibrary.TransformLocation` (`self.K2_GetComponentToWorld`) (`KismetMathLibrary.MakeVector` 0.0 (* (`self.width`) 50.0))) (`KismetMathLibrary.ComposeRotators` (`KismetMathLibrary.MakeRotator` 0.0 0.0 (select `bool` Flip :`true` 180.0 :!type "Float (single-precision)")) (`self.K2_GetComponentRotation`))))

(fn `Init`
  (params (`Wall Node Type` :type "/Game/Blueprints/NodeTypes_Wall Enum" :default "NewEnumerator0") (`Node Width` :type "Float (double-precision)" :default 20.0) (height :type "Float (double-precision)" :default 4.0) (thickness :type "Float (double-precision)" :default 0.5) (`wall seed` :type Integer))
  (locals (`Door Position WS` :type "Vector Structure" :default (0.0 0.0 0.0)) (`Door Rotation WS` :type "Rotator Structure" :default (struct)) (NewLocalVar_0 :type Integer :default 0))
  (bind _returnvalue (`self.K2_GetComponentToWorld`))
  (bind _height_of_door (`self.height of door`))
  (bind _returnvalue_2 (`KismetMathLibrary.RandomFloatInRangeFromStream` 0.8 1.2 (`self.Random Stream`)))
  (bind _returnvalue_3 (`KismetMathLibrary.RandomBoolFromStream` (`self.Random Stream`)))
  (bind _returnvalue_4 (* (`KismetMathLibrary.RandomFloatInRangeFromStream` 1.0 2.0 (`self.Random Stream`)) (`self.width of door`)))
  (set `self.width` `Node Width`)
  (set `self.height` height)
  (set `self.thickness` thickness)
  (`KismetMathLibrary.SetRandomStreamSeed` (`self.Random Stream`) `wall seed`)
  (bind _output_get (set `self.Wall Node Type` `Wall Node Type`))
  (switch `/Game/Blueprints/NodeTypes_Wall` _output_get
    (:`NewEnumerator0`
      (`self.Build Section As Wall`))
    (:`NewEnumerator1`
      (`self.Build Section As Passageway` (* (/ (`self.target block width`) 100.0) _returnvalue_2 2.0) (* (/ (`self.target block height`) 100.0) _returnvalue_2 3.0) false false _returnvalue_3))
    (:`NewEnumerator3`
      (`self.Build Section As Passageway` _returnvalue_4 _height_of_door true true _returnvalue_3))
    (:`NewEnumerator11`
      (`self.Build Section As Passageway` _returnvalue_4 _height_of_door true false _returnvalue_3))
    (:`NewEnumerator7`
      (`self.Build Section As Collapsing Wall`))
    (:`NewEnumerator12`
      (`self.Build Section As Wall`)
      (`|SpawnActorFromClass` "/Game/Blueprints/Torch.Torch_C" (`KismetMathLibrary.MakeTransform` (`KismetMathLibrary.TransformLocation` _returnvalue (* (`KismetMathLibrary.MakeVector` (`self.thickness`) (/ (`self.width`) 2.0) 2.0) 100.0)) (.rotation _returnvalue)) "Undefined" "OverrideRootScale" null null))))