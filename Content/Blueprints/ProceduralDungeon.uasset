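; Procedural dungeon generator that spawns a grid of Room actors at BeginPlay.
; BuildDungeon loops over rows and columns, spacing rooms by region width and length, with the first cell centered on the world origin.
; A random stream jitters each room on all three axes, so the layout is irregular but can be reproduced from a seed.
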(event `self.ReceiveBeginPlay`
  (`self.Build Dungeon` 3))

(fn `Build Dungeon`
  (params (Rows :type Integer :default 3) (Columns :type Integer :default 3) (`Region size x` :type "Float (double-precision)" :default 5000.0) (`Region size y` :type "Float (double-precision)" :default 5000.0))
  (locals (`Offset X` :type "Float (double-precision)") (`Offset Y` :type "Float (double-precision)"))
  (bind _output_get (set `self.REGION WIDTH` `Region size x`))
  (set `local.Offset X` (* _output_get -1.0))
  (bind _output_get_2 (set `self.REGION LENGTH` `Region size y`))
  (set `local.Offset Y` (* _output_get_2 -1.0))
  (for _index (range 1 (+ (`local.Rows`) 1))
    (for _index_2 (range 1 (+ (`local.Columns`) 1))
      (`|SpawnActorFromClass` "/Game/Blueprints/Room.Room_C" (`KismetMathLibrary.MakeTransform` (`KismetMathLibrary.MakeVector` (+ (+ (* _index (`self.REGION WIDTH`)) (`local.Offset X`)) (`KismetMathLibrary.RandomFloatInRangeFromStream` -100.0 100.0 (`self.random stream`))) (+ (+ (* _index_2 (`self.REGION LENGTH`)) (`local.Offset Y`)) (`KismetMathLibrary.RandomFloatInRangeFromStream` -100.0 100.0 (`self.random stream`))) (`KismetMathLibrary.RandomFloatInRangeFromStream` -100.0 100.0 (`self.random stream`)))) "Undefined" "OverrideRootScale" null null))))

(fn `UserConstructionScript`)