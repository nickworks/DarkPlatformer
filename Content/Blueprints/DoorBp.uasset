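; Interactable swinging door that toggles open and closed, or plays a small locked animation instead of opening when locked.
; Timelines drive the hinge's yaw, with a dot product between hinge forward and pawn direction choosing a swing away from the player.
; Init procedurally sizes the door from width and height, builds its frame from three mesh instances, and shows the lock when locked.
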(event `Try to Open the Door`
  (params (Pawn :type "Pawn Object Reference"))
  (bind (_returnvalue_x _returnvalue_y) (`KismetMathLibrary.BreakVector` (- (`self.K2_GetActorLocation` Pawn) (`self.K2_GetActorLocation`))))
  (bind _returnvalue (select `bool` (> (`KismetMathLibrary.Dot_VectorVector` (`KismetMathLibrary.Normal` (`KismetMathLibrary.MakeVector` _returnvalue_x _returnvalue_y)) (`SceneComponent.GetForwardVector` (`self.HINGE`))) 0.0) :`false` -1 :`true` 1))
  (if (not (`TimelineComponent.IsPlaying` (`self.OpenDoor`)))
    (set `self.direction` _returnvalue)
    (if (`self.isLocked`)
      (set `self.direction` _returnvalue)
      (bind (_direction _yaw) (`Timeline|Locked Animation` :!via `PlayFromStart`)
        (:`Update`
          (`SceneComponent.K2_SetRelativeRotation` (`self.HINGE`) (`KismetMathLibrary.MakeRotator` 0.0 0.0 (* _yaw (`KismetMathLibrary.Conv_IntToDouble` (`self.direction`)) 3.0)) false false)))
      (else
        (bind (_direction_2 _percent) (`Timeline|OpenDoor` :!label _label)
          (:`Update`
            (`SceneComponent.K2_SetRelativeRotation` (`self.HINGE`) (`KismetMathLibrary.MakeRotator` 0.0 0.0 (* _percent (`KismetMathLibrary.Conv_IntToDouble` (`self.direction`)) 87.0)) false false))
          (:`Finished`
            (switch `ETimelineDirection` _direction_2
              (:`Forward`
                (set `self.isOpen` true))
              (:`Backward`
                (set `self.isOpen` false)))))))))

(event `Close the Door`
  (goto _label :!via `Reverse`))

(event `/Game/Blueprints/SomethingThatCanBeInteractedWith.Player Attempted Interact`
  (params (Player :type "/Game/Blueprints/PlayerCharacter/FirstPersonCharacter Object Reference"))
  (if (`self.isOpen`)
    (`self.Close the Door`)
    (else
      (`self.Try to Open the Door` Player))))

(event `self.Lock.OnComponentActivated`
  (params (Component :type "ActorComponent Object Reference") (bReset :type Boolean)))

(fn `Init`
  (params (width :type "Float (double-precision)" :default 1.5) (height :type "Float (double-precision)" :default 3.0) (isLocked :type Boolean))
  (bind _returnvalue (- (`self.height`) 0.1))
  (bind _returnvalue_2 (- (`self.width`) 0.1))
  (bind _returnvalue_3 (- (`self.height`) 0.1))
  (bind _returnvalue_4 (- (`self.width`) 0.2))
  (bind _returnvalue_5 (`KismetMathLibrary.MakeVector` 0.0 (* _returnvalue_4 50.0) (* _returnvalue_3 50.0)))
  (set `self.width` width)
  (set `self.height` height)
  (set `self.isLocked` isLocked)
  (`SceneComponent.K2_SetRelativeLocation` (`self.HINGE`) (`KismetMathLibrary.MakeVector` 0.0 (* _returnvalue_4 -50.0)) false false)
  (`SceneComponent.K2_SetRelativeTransform` (`self.Mesh-Door`) (`KismetMathLibrary.MakeTransform` _returnvalue_5 (struct) (`KismetMathLibrary.MakeVector` 0.1 _returnvalue_4 _returnvalue_3)) false false) ; DOOR
  (`SceneComponent.K2_SetRelativeLocation` (`self.Center of Door`) _returnvalue_5 false false)
  (`SceneComponent.SetVisibility` (`self.Lock`) (`self.isLocked`) false)
  (`InstancedStaticMeshComponent.AddInstance` (`self.Mesh-Frame`) (`KismetMathLibrary.MakeTransform` (`KismetMathLibrary.MakeVector` 0.0 0.0 (* (- (`self.height`) 0.05) 100.0)) (struct) (`KismetMathLibrary.MakeVector` 0.35 (`self.width`) 0.1)))
  (`InstancedStaticMeshComponent.AddInstance` (`self.Mesh-Frame`) (`KismetMathLibrary.MakeTransform` (`KismetMathLibrary.MakeVector` 0.0 (* _returnvalue_2 -50.0) (* _returnvalue 50.0)) (struct) (`KismetMathLibrary.MakeVector` 0.35 0.1 _returnvalue)))
  (`InstancedStaticMeshComponent.AddInstance` (`self.Mesh-Frame`) (`KismetMathLibrary.MakeTransform` (`KismetMathLibrary.MakeVector` 0.0 (* _returnvalue_2 50.0) (* _returnvalue 50.0)) (struct) (`KismetMathLibrary.MakeVector` 0.35 0.1 _returnvalue))))

(fn `UserConstructionScript`)