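; Disintegrator projectile that eats away instanced-mesh pieces of any Room or Wall it hits, then destroys itself.
; On hit, it runs DestroyStuff on every InstancedStaticMeshComponent of the struck actor.
; DestroyStuff finds instances within a fixed sphere around the projectile, spawns a DisintegrationBurst effect at each transform and removes the instance.
; Removal walks indices in forward order, with a debug print; a reversed loop sits unconnected.
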(event `self.ReceiveHit`
  (params (MyComp :type "PrimitiveComponent Object Reference") (Other :type "Actor Object Reference") (OtherComp :type "PrimitiveComponent Object Reference") (bSelfMoved :type Boolean) (HitLocation :type "Vector Structure") (HitNormal :type "Vector Structure") (NormalImpulse :type "Vector Structure") (Hit :type "HitResult Structure (by ref)"))
  (cast `/Game/Blueprints/ProceduralGeneration/Room` Other
    (:`then`
      _)
    (:`CastFailed`
      (cast `/Game/Blueprints/ProceduralGeneration/Wall` Other)))
  (for _array_element (`self.K2_GetComponentsByClass` Other "/Script/Engine.InstancedStaticMeshComponent")
    (`self.Destroy Stuff` _array_element))
  (`self.K2_DestroyActor`))

(fn `Destroy Stuff`
  (params (`Instance Static Mesh` :type "InstancedStaticMeshComponent Object Reference"))
  (for _array_element (`InstancedStaticMeshComponent.GetInstancesOverlappingSphere` `Instance Static Mesh` (`self.K2_GetActorLocation`) 100.0 true)
    (`KismetSystemLibrary.PrintString` (`KismetStringLibrary.Concat_StrStr` "remove " (`KismetStringLibrary.Conv_IntToString` _array_element)))
    (bind _outinstancetransform (`InstancedStaticMeshComponent.GetInstanceTransform` (`local.Instance Static Mesh`) _array_element true))
    (`NiagaraFunctionLibrary.SpawnSystemAtLocation` "/Game/ArtStuff/Particles/DisintegrationBurst.DisintegrationBurst" (.location _outinstancetransform) (.rotation _outinstancetransform) (.scale _outinstancetransform))
    (`InstancedStaticMeshComponent.RemoveInstance` (`local.Instance Static Mesh`) _array_element)))

(fn `UserConstructionScript`
  (`parent.UserConstructionScript`))