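; CrystalProjectile is a projectile that teleports the player to a crystal platform it hits, at the cost of a Frequency Attuner.
; On hit, it casts the other actor to CrystalPlatform and asks the first-person character's InventorySystem to remove one held attuner, with damage application enabled.
; If removal succeeds, the platform teleports the character to itself and the projectile destroys itself.
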(event `self.ReceiveHit`
  (params (MyComp :type "PrimitiveComponent Object Reference") (Other :type "Actor Object Reference") (OtherComp :type "PrimitiveComponent Object Reference") (bSelfMoved :type Boolean) (HitLocation :type "Vector Structure") (HitNormal :type "Vector Structure") (NormalImpulse :type "Vector Structure") (Hit :type "HitResult Structure (by ref)"))
  (bind _ascrystal_platform (cast `/Game/Blueprints/CrystalPlatform` Other))
  (if true
    (bind _asfirst_person_character (cast `/Game/Blueprints/PlayerCharacter/FirstPersonCharacter` (`GameplayStatics.GetPlayerCharacter` 0)))
    (bind _removed_any_ (`/Game/Blueprints/PlayerCharacter/InventorySystem.Remove Item If Held` (`/Game/Blueprints/PlayerCharacter/FirstPersonCharacter.InventorySystem` _asfirst_person_character) "/Game/Blueprints/InventoryItems/ItemAbilities/FrequencyAttuner.FrequencyAttuner_C" 1 true))
    (if _removed_any_
      (`/Game/Blueprints/CrystalPlatform.Teleport Actor To Me` _ascrystal_platform _asfirst_person_character)
      (`self.K2_DestroyActor`))))

(fn `UserConstructionScript`
  (`parent.UserConstructionScript`))